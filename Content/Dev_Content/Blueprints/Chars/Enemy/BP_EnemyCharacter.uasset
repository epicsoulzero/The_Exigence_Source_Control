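; Enemy character Blueprint with a floating health-only status bar, status effects routed to its effect manager, and a stun flag.
; On death it flags IsDead on the AI blackboard, awards experience to the killer and triggers a delayed spawn from its Spawner.
; It then destroys itself and notifies the player's quest log of the kill, calling only after the quest loop completes.
; Tick draws attack-range and controller-name debug output.
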(event `self.ReceiveBeginPlay`
  (`self.UpdateHealthUI` false)
  (bind _asui_status_bar_floating (cast `/Game/Dev_Content/Blueprints/UI/Status/UI_StatusBar_Floating` (`WidgetComponent.GetWidget` (`self.UI_StatusBar`))))
  (`/Game/Dev_Content/Blueprints/UI/Status/UI_StatusBar_Floating.Initialize` _asui_status_bar_floating true false true))

(event `self.ReceiveTick`
  (params (DeltaSeconds :type "Float (single-precision)"))
  (bind (_returnvalue_x _returnvalue_y) (`KismetMathLibrary.BreakVector` (`self.K2_GetActorLocation`)))
  (bind _returnvalue (`self.GetController`))
  (`KismetSystemLibrary.DrawDebugCircle` (`KismetMathLibrary.MakeVector` _returnvalue_x _returnvalue_y 10.0) (`self.AttackRange`) 50 (struct :`R` 1.0 :`A` 1.0) 0.0 2.0 (1.0 0.0 0.0) (0.0 1.0 0.0))
  (`/Engine/EditorBlueprintResources/StandardMacros.IsValid` _returnvalue
    (:`Is Valid`
      (`KismetSystemLibrary.PrintString` (`KismetSystemLibrary.GetDisplayName` _returnvalue) true false (struct :`G` 0.66 :`B` 1.0 :`A` 1.0) 0.0))
    (:`Is Not Valid`
      (`KismetSystemLibrary.PrintString` "Hello" true false (struct :`G` 0.66 :`B` 1.0 :`A` 1.0) 0.0))))

(event `/Game/Dev_Content/Blueprints/Interfaces/BPI_StatusEffects.AddStatusEffect`
  (params (EffectToAdd :type "/Game/Dev_Content/Blueprints/Components/StatusEffects/AC_StatusEffect Object Reference"))
  (`/Game/Dev_Content/Blueprints/Components/StatusEffects/AC_StatusEffect_Manager.AddEffect` (`self.BPC_StatusEffect_Manager`) EffectToAdd))

(event `/Game/Dev_Content/Blueprints/Interfaces/BPI_StatusEffects.OnStun`
  (params (`IsStunned?` :type Boolean))
  (set `self.CanDoThings?` `IsStunned?`))

(fn `OnDeath`
  (params (Dealer :type "Actor Object Reference"))
  (bind _dealer (`local.Dealer`))
  (`BlackboardComponent.SetValueAsBool` (`AIBlueprintHelperLibrary.GetBlackboard` (`self.GetController`)) "IsDead" true)
  (`KismetSystemLibrary.PrintString` (`KismetSystemLibrary.GetDisplayName` _dealer))
  (message `/Game/Dev_Content/Blueprints/Interfaces/BPI_OnKillEffect.GainExp` _dealer 20)
  (`/Game/BP_SimpleSpawner.SpawnWithDelay_Event` (`self.Spawner`) 3.0)
  (`|ExecutionSequence`
    (:`then_0`
      (`self.K2_DestroyActor`)
      (bind _asbp_base_character (cast `/Game/Dev_Content/Blueprints/Chars/BP_BaseCharacter` (`GameplayStatics.GetPlayerCharacter` 0)))
      (for _array_element (`/Game/Dev_Content/QuestSytem/QuestLog.Quests` (`/Game/Dev_Content/Blueprints/Chars/BP_BaseCharacter.QuestLog` _asbp_base_character))
        _)
      (`/Game/Dev_Content/QuestSytem/Quest/Quest.KilledEnemy` _array_element self)
      (return))))

(fn `UserConstructionScript`)