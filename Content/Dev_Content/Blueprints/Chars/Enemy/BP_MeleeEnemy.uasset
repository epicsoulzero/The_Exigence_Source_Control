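; Melee enemy Blueprint that deals area damage around itself when its attack event fires.
; OnAttack runs a sphere overlap at AttackRange for BP_BaseCharacter actors other than itself and sends each a TakeDamageMessage with a rounded random value from DamageRange, naming its owner as dealer.
; Tick draws a red debug circle showing the attack range, while BeginPlay and construction defer to the parent class.
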(event `self.ReceiveBeginPlay`
  (`parent.ReceiveBeginPlay`))

(event `/Game/Dev_Content/Blueprints/Interfaces/BPI_CanAttack.OnAttack`
  (params (TargetActor :type "Actor Object Reference"))
  (bind (_x _y) (`KismetMathLibrary.BreakVector2D` (`self.DamageRange`)))
  (bind (_outactors _returnvalue) (`KismetSystemLibrary.SphereOverlapActors` (`self.K2_GetActorLocation`) (`self.AttackRange`) (`|MakeArray` "ObjectTypeQuery1" "ObjectTypeQuery2" "ObjectTypeQuery3" :!type "EObjectTypeQuery Enum") "/Game/Dev_Content/Blueprints/Chars/BP_BaseCharacter.BP_BaseCharacter_C" (`|MakeArray` self :!type "Actor Object Reference")))
  (if _returnvalue
    (for _array_element _outactors
      (message `/Game/Dev_Content/Blueprints/Interfaces/BPI_Damageable.TakeDamage` _array_element (`KismetMathLibrary.Conv_IntToDouble` (`KismetMathLibrary.Round` (`KismetMathLibrary.RandomFloatInRange` _x _y))) (`self.GetOwner`)))))

(event `self.ReceiveTick`
  (params (DeltaSeconds :type "Float (single-precision)"))
  (`KismetSystemLibrary.DrawDebugCircle` (`self.K2_GetActorLocation`) (`self.AttackRange`) 50 (struct :`R` 1.0 :`A` 1.0) 0.0 0.0 (1.0 0.0 0.0) (0.0 1.0 0.0) true))

(fn `UserConstructionScript`
  (`parent.UserConstructionScript`))