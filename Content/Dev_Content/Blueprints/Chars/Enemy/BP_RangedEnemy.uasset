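; BP_RangedEnemy is an enemy character Blueprint that attacks by shooting arrow projectiles in a given direction.
; ShootArrowSkill turns ProjectileSpawnPivot with a look-at rotation built from the actor's XY location and the supplied direction.
; It then spawns a BP_Projectile at ProjectileSpawnPoint, passing damage range, speed, direction and the EnemyProjectile collision profile.
; The construction script only runs the parent's logic.
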(event `/Game/Dev_Content/Blueprints/Interfaces/BPI_ShootArrowSkill.ShootArrowSkill`
  (params (Direction :type "Vector Structure"))
  (bind (_returnvalue_x _returnvalue_y) (`KismetMathLibrary.BreakVector` (`self.K2_GetActorLocation`)))
  (bind (_x _y _z) (`KismetMathLibrary.BreakVector3f` Direction))
  (`SceneComponent.K2_SetWorldRotation` (`self.ProjectileSpawnPivot`) (`KismetMathLibrary.FindLookAtRotation` (`KismetMathLibrary.MakeVector` _returnvalue_x _returnvalue_y _z) (+ (`KismetMathLibrary.MakeVector` _returnvalue_x _returnvalue_y _z) (`KismetMathLibrary.MakeVector` _x _y _z))) false true)
  (`|SpawnActorFromClass` "/Game/Dev_Content/Blueprints/Miscellaneous/BP_Projectile.BP_Projectile_C" (`KismetMathLibrary.MakeTransform` (`SceneComponent.K2_GetComponentLocation` (`self.ProjectileSpawnPoint`))) "AlwaysSpawn" "OverrideRootScale" null (2.0 5.0) 750.0 Direction "EnemyProjectile" null))

(fn `UserConstructionScript`
  (`parent.UserConstructionScript`))