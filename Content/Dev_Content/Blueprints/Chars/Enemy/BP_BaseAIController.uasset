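; Base AI controller for enemy characters that starts each enemy's own behavior tree.
; After a half-second delay from BeginPlay, it caches the possessed BP_EnemyCharacter, runs that character's behavior tree and copies its attack range and speed into the blackboard.
; With debugging enabled, Tick mirrors the pawn's CanDoThings flag to the blackboard, and a failed tree start prints an on-screen message.
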(event `self.ReceiveBeginPlay`
  (`self.DelayedBeginPlay`))

(event `self.ReceiveTick`
  (params (DeltaSeconds :type "Float (single-precision)"))
  (if (`self.ShowDebugs?`)
    (`BlackboardComponent.SetValueAsBool` (`AIBlueprintHelperLibrary.GetBlackboard` null) "CanDoThings?" (`/Game/Dev_Content/Blueprints/Chars/Enemy/BP_EnemyCharacter.CanDoThings?` (cast `/Game/Dev_Content/Blueprints/Chars/Enemy/BP_EnemyCharacter` (`self.K2_GetPawn`) :!pure true)))))

(event `DelayedBeginPlay`
  (`KismetSystemLibrary.Delay` 0.5)
  (bind _asbp_enemy_character (cast `/Game/Dev_Content/Blueprints/Chars/Enemy/BP_EnemyCharacter` (`self.K2_GetPawn`)))
  (bind _output_get (set `self.EnemyBPRef` _asbp_enemy_character))
  (bind _returnvalue (`self.RunBehaviorTree` (`/Game/Dev_Content/Blueprints/Chars/Enemy/BP_EnemyCharacter.BehaviorTreeRef` _output_get)))
  (if _returnvalue
    (`BlackboardComponent.SetValueAsFloat` (`AIBlueprintHelperLibrary.GetBlackboard` null) "AttackRange" (`/Game/Dev_Content/Blueprints/Chars/Enemy/BP_EnemyCharacter.AttackRange` (`self.EnemyBPRef`)))
    (`BlackboardComponent.SetValueAsFloat` (`AIBlueprintHelperLibrary.GetBlackboard` null) "AttackSpeed" (`/Game/Dev_Content/Blueprints/Chars/Enemy/BP_EnemyCharacter.AttackSpeed` (`self.EnemyBPRef`)))
    (set `self.Init?` true)
    (else
      (`KismetSystemLibrary.PrintString` "Running Behavior tree failed" (`self.ShowDebugs?`) false (struct :`G` 0.66 :`B` 1.0 :`A` 1.0) 10.0))))

(fn `UserConstructionScript`)