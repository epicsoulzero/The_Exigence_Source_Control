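; Parent Blueprint for NPCs that forwards player interaction to every quest in the player's quest log.
; An outer NoFireZone flags the player controller to disable attacks, and BoxCollision shows the name, highlights the mesh and stops movement.
; Leaving the box clears the highlight and zooms the camera out if dialog is open.
; The click handler is empty, and the dialog-opening zoom and fade logic is disconnected.
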(event `self.ReceiveBeginPlay`
  (`SceneComponent.SetVisibility` (`self.NPC Name`) false false))

(event `/Game/Dev_Content/QuestSytem/InteractInterface.Interact`
  (bind _asbp_base_character (cast `/Game/Dev_Content/Blueprints/Chars/BP_BaseCharacter` (`GameplayStatics.GetPlayerCharacter` 0)))
  (for _array_element (`/Game/Dev_Content/QuestSytem/QuestLog.Quests` (`/Game/Dev_Content/Blueprints/Chars/BP_BaseCharacter.QuestLog` _asbp_base_character))
    (`/Game/Dev_Content/QuestSytem/Quest/Quest.Interacted` _array_element self)))

(event `self.NoFireZone.OnComponentBeginOverlap`
  (params (OverlappedComponent :type "PrimitiveComponent Object Reference") (OtherActor :type "Actor Object Reference") (OtherComp :type "PrimitiveComponent Object Reference") (OtherBodyIndex :type Integer) (bFromSweep :type Boolean) (SweepResult :type "HitResult Structure (by ref)"))
  ;[1 1 1] For Disabling Attack at NPC Trigger Box + Stop Movement
  (bind _asbp_player_controller (cast `/Game/Dev_Content/Blueprints/Chars/Player/BP_PlayerController` (`GameplayStatics.GetPlayerController` 0)))
  (set `/Game/Dev_Content/Blueprints/Chars/Player/BP_PlayerController.NpcBoxOverlap` true _asbp_player_controller))

(event `self.Box Collision.OnComponentBeginOverlap`
  (params (OverlappedComponent :type "PrimitiveComponent Object Reference") (OtherActor :type "Actor Object Reference") (OtherComp :type "PrimitiveComponent Object Reference") (OtherBodyIndex :type Integer) (bFromSweep :type Boolean) (SweepResult :type "HitResult Structure (by ref)"))
  (`SceneComponent.SetVisibility` (`self.NPC Name`) true false)
  (`MeshComponent.SetScalarParameterValueOnMaterials` (`self.Mesh`) "selected" 1.0)
  (set `self.BoxOverlapped?` true)
  (`Controller.StopMovement` (stale `self.NoFireZone.OnComponentBeginOverlap` _asbp_player_controller)))

(event `self.Box Collision.OnComponentEndOverlap`
  (params (OverlappedComponent :type "PrimitiveComponent Object Reference") (OtherActor :type "Actor Object Reference") (OtherComp :type "PrimitiveComponent Object Reference") (OtherBodyIndex :type Integer))
  (`SceneComponent.SetVisibility` (`self.NPC Name`) false false)
  (`MeshComponent.SetScalarParameterValueOnMaterials` (`self.Mesh`) "selected" 0.0)
  (if (`self.DialogOpen?`)
    (bind _asbp_player_character (cast `/Game/Dev_Content/Blueprints/Chars/Player/BP_PlayerCharacter` (`GameplayStatics.GetPlayerCharacter` 0)))
    (`/Game/Dev_Content/Blueprints/Chars/Player/BP_PlayerCharacter.HeightCameraChanger` _asbp_player_character (`self.ZoomOut`))
    (set `self.BoxOverlapped?` false)
    (set `self.DialogOpen?` false)))

(event `self.NoFireZone.OnComponentEndOverlap`
  (params (OverlappedComponent :type "PrimitiveComponent Object Reference") (OtherActor :type "Actor Object Reference") (OtherComp :type "PrimitiveComponent Object Reference") (OtherBodyIndex :type Integer))
  ;[1 1 1] For Enabling Attack at NPC Trigger Box
  (bind _asbp_player_controller (cast `/Game/Dev_Content/Blueprints/Chars/Player/BP_PlayerController` (`GameplayStatics.GetPlayerController` 0)))
  (set `/Game/Dev_Content/Blueprints/Chars/Player/BP_PlayerController.NpcBoxOverlap` false _asbp_player_controller))

(event `QuickFadeToBlack`
  (bind _returnvalue (`|CreateWidget` "/Game/Dev_Content/Blueprints/Chars/NPC/BlackScreenPop.BlackScreenPop_C" (`GameplayStatics.GetPlayerController` 0)))
  (bind _output_get (set `self.BlackScreenPop` _returnvalue))
  (`UserWidget.AddToViewport` _output_get 0)
  (`KismetSystemLibrary.Delay` 1.0)
  (`Widget.RemoveFromParent` _output_get))

(event `self.Mesh.OnClicked`
  (params (TouchedComponent :type "PrimitiveComponent Object Reference") (ButtonPressed :type "Key Structure")))

(fn `UserConstructionScript`)