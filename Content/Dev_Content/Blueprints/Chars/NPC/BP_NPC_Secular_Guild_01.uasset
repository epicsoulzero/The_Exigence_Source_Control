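; Secular guild NPC that opens a dialogue widget when the player clicks its mesh.
; The click only works while BoxOverlapped is true, a flag this graph reads but never sets.
; It creates NPC_Dialogue_TheSecular01, starts it with ConversationInfo and adds it to the viewport.
; Ending overlap with BoxCollision removes the open dialogue and clears its open flag.
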(event `self.Box Collision.OnComponentEndOverlap`
  (params (OverlappedComponent :type "PrimitiveComponent Object Reference") (OtherActor :type "Actor Object Reference") (OtherComp :type "PrimitiveComponent Object Reference") (OtherBodyIndex :type Integer))
  (if (`self.DialogOpenTheSecular?`)
    (`Widget.RemoveFromParent` (stale `self.Mesh.OnClicked` _returnvalue))
    (set `self.DialogOpenTheSecular?` false)))

(event `self.Mesh.OnClicked`
  (params (TouchedComponent :type "PrimitiveComponent Object Reference") (ButtonPressed :type "Key Structure"))
  (if (`self.BoxOverlapped?`)
    (bind _returnvalue (`|CreateWidget` "/Game/Dev_Content/Blueprints/Chars/NPC/NPC_Dialogue_TheSecular01.NPC_Dialogue_TheSecular01_C"))
    (`/Game/Dev_Content/Blueprints/Chars/NPC/NPC_Dialogue_TheSecular01.Begin Secular` _returnvalue (`self.ConversationInfo`))
    (`UserWidget.AddToViewport` _returnvalue 0)
    (set `self.DialogOpenTheSecular?` true)))

(fn `UserConstructionScript`
  (`parent.UserConstructionScript`))