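; BP_NPC_Story is a story NPC that the player clicks to start a conversation.
; Clicking the mesh while BoxOverlapped is set creates an NPC_Dialogue_Story widget, starts it with ConversationInfo and adds it to the viewport.
; When an overlap with the collision box ends, any open dialogue is removed from screen.
; BeginPlay and the construction script only call the parent.
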(event `self.ReceiveBeginPlay`
  (`parent.ReceiveBeginPlay`))

(event `self.Box Collision.OnComponentEndOverlap`
  (params (OverlappedComponent :type "PrimitiveComponent Object Reference") (OtherActor :type "Actor Object Reference") (OtherComp :type "PrimitiveComponent Object Reference") (OtherBodyIndex :type Integer))
  (if (`self.DialogOpenStory?`)
    (`Widget.RemoveFromParent` (stale `self.Mesh.OnClicked` _returnvalue))
    (set `self.DialogOpenStory?` false)))

(event `self.Mesh.OnClicked`
  (params (TouchedComponent :type "PrimitiveComponent Object Reference") (ButtonPressed :type "Key Structure"))
  (if (`self.BoxOverlapped?`)
    (bind _returnvalue (`|CreateWidget` "/Game/Dev_Content/Blueprints/Chars/NPC/NPC_Dialogue_Story.NPC_Dialogue_Story_C"))
    (bind _output_get (set `self.DialogStory` _returnvalue))
    (`/Game/Dev_Content/Blueprints/Chars/NPC/NPC_Dialogue_Story.Begin Story` _output_get (`self.ConversationInfo`))
    (`UserWidget.AddToViewport` _output_get 0)
    (set `self.DialogOpenStory?` true)))

(fn `UserConstructionScript`
  (`parent.UserConstructionScript`))