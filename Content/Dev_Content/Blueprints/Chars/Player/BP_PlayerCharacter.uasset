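; Player character Blueprint for a Hunter with a pet, handling skills, stats, experience, damage and death.
; Skill events aim an arrow pivot and call skill components, most attacks using level-scaled StatsSystem damage, though Multishot uses unscaled damage.
; StatsSystem sets health and mana maximums shown on the status HUD, and reduces incoming damage.
; Experience triggers level-ups, death kills the pet and respawns through a spawner, and debug keys force levels or death.
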(event `self.ReceiveBeginPlay`
  (`|ExecutionSequence`
    (:`then_0`
      (`self.Initialize_UI_HUD`))
    (:`then_2`
      (`parent.ReceiveBeginPlay`))))

(event `/Game/Dev_Content/Blueprints/Interfaces/BPI_OnKillEffect.GainExp`
  (params (Amount :type Integer))
  (`self.ManageExpGained` Amount))

(event `/Game/Dev_Content/Blueprints/Interfaces/BPI_StatusEffects.AddStatusEffect`
  (params (EffectToAdd :type "/Game/Dev_Content/Blueprints/Components/StatusEffects/AC_StatusEffect Object Reference"))
  (`/Game/Dev_Content/Blueprints/Components/StatusEffects/AC_StatusEffect_Manager.AddEffect` (`self.StatusEffectManager`) EffectToAdd))

(event `HeightCameraChanger`
  (params (HeightChanger :type "Vector Structure"))
  (`SceneComponent.K2_SetRelativeLocation` (`self.Camera`) HeightChanger false true))

(event `RotatorCameraChanger`
  (params (RotationChanger :type "Rotator Structure"))
  (`SceneComponent.K2_SetRelativeRotation` (`self.Camera`) RotationChanger false false))

(event `Key|Seven`
  (params (Key :type "Key Structure"))
  (:`Pressed`
    (`self.ForceLevelUp`)
    (`self.UpdateAllStats`)))

(event `Key|Eight`
  (params (Key :type "Key Structure"))
  (:`Pressed`
    (`self.ForceLevelDown`)
    (`self.UpdateAllStats`)))

(event `Key|Tab`
  (params (Key :type "Key Structure"))
  (:`Pressed`
    (set `self.ShowStats?` (not (`self.ShowStats?`)))))

(event `Key|BackSpace`
  (params (Key :type "Key Structure"))
  (:`Pressed`
    (`/Game/Dev_Content/Blueprints/Interfaces/BPI_Damageable.TakeDamage` 99999.0)
    (`self.OnDeath` null)))

(event `/Game/Dev_Content/Blueprints/Interfaces/BPI_HunterSkills.UseHunterBasic`
  (params (Direction :type "Vector Structure"))
  (bind (_min _max) (`self.GetScaledDamage`))
  ;[1 1 1] Hunter Basic Attack
  (`SceneComponent.K2_SetWorldRotation` (`self.ArrowSpawnPivot`) (`self.RotateToTargetDir` Direction) false true)
  (`|ExecutionSequence`
    (:`then_0`
      (set `/Game/Dev_Content/Blueprints/Components/Skills/AC_HunterBasic.Damage` (`KismetMathLibrary.MakeVector2D` _min _max) (`self.Hunter_Skill`)))
    (:`then_1`
      (`/Game/Dev_Content/Blueprints/Components/Skills/AC_HunterBasic.UseSkill` (`self.Hunter_Skill`) self Direction (`SceneComponent.K2_GetComponentLocation` (`self.ArrowSpawnPoint`))))))

(event `/Game/Dev_Content/Blueprints/Interfaces/BPI_HunterSkills.UseMultiShot`
  (params (Direction :type "Vector Structure"))
  (bind (_mindamage _maxdamage) (`/Game/Dev_Content/Blueprints/Components/AC_StatsSystem.GetDamage` (`self.StatsSystem`)))
  ;[1 1 1] Multishot Skill
  (`SceneComponent.K2_SetWorldRotation` (`self.ArrowSpawnPivot`) (`self.RotateToTargetDir` Direction) false true)
  (`|ExecutionSequence`
    (:`then_0`
      (set `/Game/Dev_Content/Blueprints/Components/Skills/AC_MultiShot_Skill.Damage` (`KismetMathLibrary.MakeVector2D` (`KismetMathLibrary.Conv_IntToDouble` _mindamage) (`KismetMathLibrary.Conv_IntToDouble` _maxdamage)) (`self.Multishot_Skill`)))
    (:`then_1`
      (`/Game/Dev_Content/Blueprints/Components/Skills/AC_MultiShot_Skill.UseSkill` (`self.Multishot_Skill`) self Direction (`SceneComponent.K2_GetComponentLocation` (`self.ArrowSpawnPoint`))))))

(event `/Game/Dev_Content/Blueprints/Interfaces/BPI_HunterSkills.UseExplosiveShot`
  (params (Direction :type "Vector Structure"))
  (bind (_min _max) (`self.GetScaledDamage`))
  ;[1 1 1] Explosive Shot Skill
  (`SceneComponent.K2_SetWorldRotation` (`self.ArrowSpawnPivot`) (`self.RotateToTargetDir` Direction) false true)
  (`|ExecutionSequence`
    (:`then_0`
      (set `/Game/Dev_Content/Blueprints/Components/Skills/AC_ExplosiveShot_Skill.InitialDamage` (`KismetMathLibrary.MakeVector2D` _min _max) (`self.ExplosiveShot_Skill`)))
    (:`then_1`
      (`/Game/Dev_Content/Blueprints/Components/Skills/AC_ExplosiveShot_Skill.UseSkill` (`self.ExplosiveShot_Skill`) self Direction (`SceneComponent.K2_GetComponentLocation` (`self.ArrowSpawnPoint`))))))

(event `/Game/Dev_Content/Blueprints/Interfaces/BPI_HunterSkills.UseRushScent`
  ;[1 1 1] Rush Scent Skill
  (`/Game/Dev_Content/Blueprints/Components/Skills/AC_RushScent_Skill.UseSkill` (`self.RushScent_Skill`) self))

(event `/Game/Dev_Content/Blueprints/Interfaces/BPI_HunterSkills.UseTrap`
  (params (HitPoint :type "Vector Structure") (Direction :type "Vector Structure"))
  ;[1 1 1] Trap Skill
  (`SceneComponent.K2_SetWorldRotation` (`self.ArrowSpawnPivot`) (`self.RotateToTargetDir` Direction) false true)
  (`/Game/Dev_Content/Blueprints/Components/Skills/AC_Trap_Skill.UseSkill` (`self.Trap_Skill`) self HitPoint (`SceneComponent.K2_GetComponentLocation` (`self.ArrowSpawnPoint`))))

(event `/Game/Dev_Content/Blueprints/Interfaces/BPI_HunterSkills.UseVolleyShot`
  (params (HitPoint :type "Vector Structure"))
  (bind (_min _max) (`self.GetScaledDamage`))
  ;[1 1 1] Volley Shot Skill
  (set `/Game/Dev_Content/Blueprints/Components/Skills/AC_VolleyShot_Skill.Damage` (`KismetMathLibrary.MakeVector2D` _min _max) (`self.VolleyShot_Skill`))
  (`/Game/Dev_Content/Blueprints/Components/Skills/AC_VolleyShot_Skill.UseSkill` (`self.VolleyShot_Skill`) self HitPoint))

(event `/Game/Dev_Content/Blueprints/Interfaces/BPI_HunterSkills.UsePetCharge`
  (params (HitTarget :type "Actor Object Reference") (HitLocation :type "Vector Structure"))
  (`/Game/Dev_Content/Blueprints/Components/Skills/NotDone/AC_PetCharge_Skill.UseSkill` (`self.PetCharge_Skill`) self HitTarget HitLocation))

(event `/Game/Dev_Content/Blueprints/Interfaces/BPI_HunterSkills.UseDamageBuff`
  ;[1 1 1] Buff Skills
  (`/Game/Dev_Content/Blueprints/Components/Skills/AC_DamageUp_Skill.UseSkill` (`self.DamageUp_Skill`) self))

(event `/Game/Dev_Content/Blueprints/Interfaces/BPI_HunterSkills.UseDefenseBuff`
  ;[1 1 1] Buff Skills
  (`/Game/Dev_Content/Blueprints/Components/Skills/AC_DefenseUp_Skill.UseSkill` (`self.DefenseUp_Skill`) self))

(fn `DebugStats`
  (locals (TextColor :type "LinearColor Structure" :default (struct :`G` 1.0 :`B` 0.02864 :`A` 1.0)) (LineColor :type "LinearColor Structure" :default (struct :`R` 1.0 :`G` 0.740053 :`A` 1.0)))
  (bind (_strength _agility _intellect) (`/Game/Dev_Content/Blueprints/Components/AC_StatsSystem.GetPrimaryStats` (`self.StatsSystem`)))
  (bind (_mindamage _maxdamage) (`/Game/Dev_Content/Blueprints/Components/AC_StatsSystem.GetDamage` (`self.StatsSystem`)))
  (`|ExecutionSequence`
    (:`then_0`
      (`|ExecutionSequence`
        (:`then_0`
          (`KismetSystemLibrary.PrintString` "----------------------------------" true false (`local.LineColor`) 0.0)
          (`KismetSystemLibrary.PrintString` (`KismetStringLibrary.Concat_StrStr` "Max HP: " (`KismetStringLibrary.Conv_IntToString` (`/Game/Dev_Content/Blueprints/Components/AC_StatsSystem.GetHealth` (`self.StatsSystem`))) " | Max Energy: " (`KismetStringLibrary.Conv_IntToString` (`/Game/Dev_Content/Blueprints/Components/AC_StatsSystem.GetEnergy` (`self.StatsSystem`)))) true false (`local.TextColor`) 0.0))
        (:`then_1`
          (`KismetSystemLibrary.PrintString` "DEFENSIVE STATS" true false (`local.TextColor`) 0.0))))
    (:`then_1`
      (`|ExecutionSequence`
        (:`then_0`
          (`KismetSystemLibrary.PrintString` "----------------------------------" true false (`local.LineColor`) 0.0)
          (`KismetSystemLibrary.PrintString` (`KismetStringLibrary.Concat_StrStr` "Damage: " (`KismetStringLibrary.Concat_StrStr` (`KismetStringLibrary.Conv_IntToString` _mindamage) " - " (`KismetStringLibrary.Conv_IntToString` _maxdamage)) " | Atk Speed: " (`KismetStringLibrary.Conv_DoubleToString` (`/Game/Dev_Content/Blueprints/Components/AC_StatsSystem.GetAttackSpeed` (`self.StatsSystem`))) " | Crit Chance: " (`KismetStringLibrary.Conv_DoubleToString` (`/Game/Dev_Content/Blueprints/Components/AC_StatsSystem.GetCritChance` (`self.StatsSystem`)))) true false (`local.TextColor`) 0.0))
        (:`then_1`
          (`KismetSystemLibrary.PrintString` "OFFENSIVE STATS" true false (`local.TextColor`) 0.0))))
    (:`then_2`
      (`|ExecutionSequence`
        (:`then_0`
          (`KismetSystemLibrary.PrintString` "----------------------------------" true false (`local.LineColor`) 0.0)
          (`KismetSystemLibrary.PrintString` (`KismetStringLibrary.Concat_StrStr` "Str: " (`KismetStringLibrary.Conv_IntToString` _strength) " | Agi: " (`KismetStringLibrary.Conv_IntToString` _agility) " | Int: " (`KismetStringLibrary.Conv_IntToString` _intellect)) true false (`local.TextColor`) 0.0))
        (:`then_1`
          (`KismetSystemLibrary.PrintString` "PRIMARY STATS" true false (`local.TextColor`) 0.0))))))

(fn `GetScaledDamage`
  (returns (Min :type "Float (double-precision)") (Max :type "Float (double-precision)"))
  (bind _out (`self.GetLevelMultiplier`))
  (bind (_mindamage _maxdamage) (`/Game/Dev_Content/Blueprints/Components/AC_StatsSystem.GetDamage` (`self.StatsSystem`)))
  (return (`KismetMathLibrary.Conv_IntToDouble` (`KismetMathLibrary.Round` (* _mindamage _out))) (`KismetMathLibrary.Conv_IntToDouble` (`KismetMathLibrary.Round` (* _maxdamage _out)))))

(fn `Initialize_UI_HUD`
  (`|ExecutionSequence`
    (:`then_0`
      (bind _returnvalue (`|CreateWidget` "/Game/Dev_Content/Blueprints/UI/Status/UI_PlayerStatus_HUD.UI_PlayerStatus_HUD_C" (`GameplayStatics.GetPlayerController` 0)))
      (bind _output_get (set `self.Ref_Status_HUD` _returnvalue))
      (`UserWidget.AddToViewport` _output_get 0)
      (bind _output_get_2 (set `self.ExpReq` (`self.BaseExpReq`)))
      (`/Game/Dev_Content/Blueprints/UI/Status/UI_PlayerStatus_HUD.UpdateExp` (`self.Ref_Status_HUD`) _output_get_2 (`self.CurrentExp`) true)
      (`self.UpdateAllStats`))))

(fn `ManageExpGained`
  (params (Amount :type Integer))
  (`|ExecutionSequence`
    (:`then_0`
      (bind _output_get (set `self.CurrentExp` (+ (`local.Amount`) (`self.CurrentExp`))))
      (`/Game/Dev_Content/Blueprints/UI/Status/UI_PlayerStatus_HUD.UpdateExp` (`self.Ref_Status_HUD`) (`self.ExpReq`) _output_get true))
    (:`then_1`
      (if (>= (`self.CurrentExp`) (`self.ExpReq`))
        (`self.ForceLevelUp`)
        (set `self.CurrentExp` (- (`self.CurrentExp`) (`self.ExpReq`)))
        (set `self.ExpReq` (`KismetMathLibrary.FTrunc` (* (`self.ExpMultiplier`) (`self.ExpReq`))))))))

(fn `OnDeath`
  (params (Dealer :type "Actor Object Reference"))
  (`|ExecutionSequence`
    (:`then_0`
      (`/Game/Dev_Content/Blueprints/Components/Skills/AC_PetSystem.KillPet` (`self.PetSys`) (`local.Dealer`)))
    (:`then_1`
      (`/Game/BP_SimpleSpawner.SpawnWithDelay_Event` (`self.Spawner`) 2.0)
      (`self.K2_DestroyActor`))))

(fn `TakeDamage`
  (params (DamageAmount :type "Float (double-precision)") (Dealer :type "Actor Object Reference"))
  (returns (IsDead :type Boolean))
  (bind _isdead (`parent.TakeDamage` (* DamageAmount (- 1.0 (`/Game/Dev_Content/Blueprints/Components/AC_StatsSystem.GetDamageReduction` (`self.StatsSystem`)))) Dealer))
  (return _isdead))

(fn `UpdateAllStats`
  (`|ExecutionSequence`
    (:`then_0`
      (`/Game/Dev_Content/Blueprints/Components/AC_HealthSystem.SetMaxHealth` (`self.HealthSys`) (`KismetMathLibrary.Conv_IntToDouble` (`/Game/Dev_Content/Blueprints/Components/AC_StatsSystem.GetHealth` (`self.StatsSystem`))) true)
      (`self.UpdateHealthUI` true))
    (:`then_1`
      (`/Game/Dev_Content/Blueprints/Components/AC_ManaSystem.SetMaxMana` (`self.ManaSys`) (`KismetMathLibrary.Conv_IntToDouble` (`/Game/Dev_Content/Blueprints/Components/AC_StatsSystem.GetEnergy` (`self.StatsSystem`))) true)
      (`self.UpdateManaUI` true))))

(fn `UpdateHealthUI`
  (params (`Notify?` :type Boolean))
  (bind (_maxhealth _currenthealth) (`/Game/Dev_Content/Blueprints/Components/AC_HealthSystem.GetHealthStats` (`self.HealthSys`)))
  (`/Game/Dev_Content/Blueprints/UI/Status/UI_PlayerStatus_HUD.UpdateHealth` (`self.Ref_Status_HUD`) (`KismetMathLibrary.FTrunc` _maxhealth) (`KismetMathLibrary.FTrunc` _currenthealth) (`local.Notify?`)))

(fn `UpdateManaUI`
  (params (`Notify?` :type Boolean))
  (bind (_maxmana _currentmana) (`/Game/Dev_Content/Blueprints/Components/AC_ManaSystem.GetManaStats` (`self.ManaSys`)))
  (`/Game/Dev_Content/Blueprints/UI/Status/UI_PlayerStatus_HUD.UpdateMana` (`self.Ref_Status_HUD`) (`KismetMathLibrary.FTrunc` _maxmana) (`KismetMathLibrary.FTrunc` _currentmana) `Notify?`))

(fn `UseRapidFireShot`
  (params (Direction :type "Vector Structure"))
  (returns (`Success?` :type Boolean))
  (bind (_min _max) (`self.GetScaledDamage`))
  (`SceneComponent.K2_SetWorldRotation` (`self.ArrowSpawnPivot`) (`self.RotateToTargetDir` Direction) false true)
  (set `/Game/Dev_Content/Blueprints/Components/Skills/AC_RapidFireShot_Skill.Damage Min Max` (`KismetMathLibrary.MakeVector2D` _min _max) (`self.RapidFireShot_Skill`))
  (bind _return (`/Game/Dev_Content/Blueprints/Components/Skills/AC_RapidFireShot_Skill.UseSkill` (`self.RapidFireShot_Skill`) self (`SceneComponent.K2_GetComponentLocation` (`self.ArrowSpawnPoint`)) (`local.Direction`)))
  (return _return))

(fn `UserConstructionScript`
  (`parent.UserConstructionScript`))