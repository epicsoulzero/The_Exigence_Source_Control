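; Base character Blueprint providing health, mana, levels and proximity interaction for quests.
; HealthSys and ManaSys feed a floating status bar, while TakeDamage also spawns floating text and destroys the actor on death.
; InteractionField overlaps attach a prompt widget, and the Interaction input opens quests and zooms the player camera.
; Tick resets camera height outside the field and halts movement during quest UI; older dialogue and quest-widget logic is disconnected.
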(event `self.ReceiveBeginPlay`
  (`self.UpdateHealthUI` false)
  (`self.UpdateManaUI` false)
  (bind _asui_status_bar_floating (cast `/Game/Dev_Content/Blueprints/UI/Status/UI_StatusBar_Floating` (`WidgetComponent.GetWidget` (`self.UI_StatusBar`))))
  (`/Game/Dev_Content/Blueprints/UI/Status/UI_StatusBar_Floating.Initialize` _asui_status_bar_floating true true true))

(event `self.InteractionField.OnComponentBeginOverlap`
  (params (OverlappedComponent :type "PrimitiveComponent Object Reference") (OtherActor :type "Actor Object Reference") (OtherComp :type "PrimitiveComponent Object Reference") (OtherBodyIndex :type Integer) (bFromSweep :type Boolean) (SweepResult :type "HitResult Structure (by ref)"))
  (`/Game/Dev_Content/QuestSytem/QuestMacros.CheckForInteraction` OtherActor
    (:`True`
      _)
    (:`Interact`
      _))
  (bind _returnvalue (`AddComponent|NODE_AddWidgetComponent-0`))
  (set `self.InteractMessage` _returnvalue)
  (`SceneComponent.K2_AttachToComponent` _returnvalue OtherComp "None" "KeepRelative" "KeepRelative" "KeepRelative" true)
  (set `self.IsInsideInteractionField` true))

(event `self.InteractionField.OnComponentEndOverlap`
  (params (OverlappedComponent :type "PrimitiveComponent Object Reference") (OtherActor :type "Actor Object Reference") (OtherComp :type "PrimitiveComponent Object Reference") (OtherBodyIndex :type Integer))
  (`|ExecutionSequence`
    (:`then_0`
      (bind _interactmessage (`self.InteractMessage`)
        (:`then`
          (`ActorComponent.K2_DestroyComponent` _interactmessage)
          (set `self.InteractMessage` null))
        (:`else`)))
    (:`then_2`
      (if (`self.QuestUIOpen`)
        (`self.QFB+HCC-N`)
        (set `self.QuestUIOpen` false)))
    (:`then_3`
      (set `self.IsInsideInteractionField` false))))

(event `Base Quest`)

(event `InputAction|Interaction`
  (params (Key :type "Key Structure"))
  (:`Pressed`
    (`|ExecutionSequence`
      (:`then_0`
        (bind _interactmessage (`self.InteractMessage`)
          (:`then`
            (bind _returnvalue (`ActorComponent.GetOwner` (`SceneComponent.GetAttachParent` _interactmessage)))
            (bind _quest (`/Game/Dev_Content/QuestSytem/QuestMacros.CheckForInteraction` _returnvalue)
              (:`True`
                (`/Game/Dev_Content/QuestSytem/QuestMacros.DisplayQuests` _quest
                  (:`Out`
                    _)))
              (:`Interact`
                (message `/Game/Dev_Content/QuestSytem/InteractInterface.Interact` _returnvalue)))
            (set `self.QuestUIOpen` true))
          (:`else`)))
      (:`then_1`
        (`SceneComponent.SetVisibility` (`self.InteractMessage`) false false))
      (:`then_2`
        (bind _asbp_player_character (cast `/Game/Dev_Content/Blueprints/Chars/Player/BP_PlayerCharacter` (`GameplayStatics.GetPlayerCharacter` 0)))
        (`/Game/Dev_Content/Blueprints/Chars/Player/BP_PlayerCharacter.HeightCameraChanger` _asbp_player_character (`self.ZoomIn`))
        (`MeshComponent.SetScalarParameterValueOnMaterials` (`self.Mesh`) "selected" 0.0)))))

(event `QuickFadeToBlack`
  (bind _returnvalue (`|CreateWidget` "/Game/Dev_Content/Blueprints/Chars/NPC/BlackScreenPop.BlackScreenPop_C" (`GameplayStatics.GetPlayerController` 0)))
  (bind _output_get (set `self.BlackScreenPop` _returnvalue))
  (`UserWidget.AddToViewport` _output_get 0)
  (`KismetSystemLibrary.Delay` 1.0))

(event `QFB+HCC-N`
  (`self.QuickFadeToBlack`)
  (bind _asbp_player_character (cast `/Game/Dev_Content/Blueprints/Chars/Player/BP_PlayerCharacter` (`GameplayStatics.GetPlayerCharacter` 0) :!label _label))
  (`/Game/Dev_Content/Blueprints/Chars/Player/BP_PlayerCharacter.HeightCameraChanger` _asbp_player_character (0.0 0.0 0.0)))

(event `OCEOVIF`
  (goto _label))

(event `self.ManaSys.OnCurrentManaChanged`
  (`self.UpdateManaUI` false))

(event `self.ReceiveTick`
  (params (DeltaSeconds :type "Float (single-precision)"))
  (`|ExecutionSequence`
    (:`then_0`
      (if (not (`self.IsInsideInteractionField`))
        (`self.OCEOVIF`)))
    (:`then_1`
      (if (`self.QuestUIOpen`)
        (`NavMovementComponent.StopActiveMovement` (`self.CharacterMovement`))))))

(fn `Add_MenuToViewport`
  (returns (Success :type Boolean))
  (return false))

(fn `Construct_MenuSystem`
  (returns (Success :type Boolean))
  (return false))

(fn `ForceLevelDown`
  (bind _returnvalue (- (`self.Level`) 1))
  (if (>= _returnvalue 1)
    (bind _output_get (set `self.Level` _returnvalue))
    (`KismetSystemLibrary.PrintString` (`KismetStringLibrary.Concat_StrStr` "LEVEL DOWN: " (`KismetStringLibrary.Conv_IntToString` _output_get)))))

(fn `ForceLevelUp`
  (bind _output_get (set `self.Level` (+ (`self.Level`) 1)))
  (`KismetSystemLibrary.PrintString` (`KismetStringLibrary.Concat_StrStr` "LEVEL UP: " (`KismetStringLibrary.Conv_IntToString` _output_get)) true false (struct :`G` 0.66 :`B` 1.0 :`A` 1.0) 10.0))

(fn `Get_Current_MenuType`
  (returns (ReturnValue :type "/Game/UltimateMenu/Blueprints/Data/Enums/Enum_MenuHandlerType Enum"))
  (return "NewEnumerator2"))

(fn `Get_Master_Widget`
  (returns (ReturnValue :type "/Game/UltimateMenu/UserInterface/WB_MenuMaster Object Reference"))
  (return null))

(fn `GetLevelMultiplier`
  (returns (Out :type "Float (double-precision)"))
  (return (+ (* (`self.LevelMultiplier`) (- (`self.Level`) 1)) 1.0)))

(fn `OnDeath`
  (params (Dealer :type "Actor Object Reference"))
  (`self.K2_DestroyActor`)
  (return))

(fn `SpawnFloatingText`
  (params (Text :type Text))
  (`|SpawnActorFromClass` "/Game/Dev_Content/Blueprints/Miscellaneous/BP_FloatingText.BP_FloatingText_C" (`KismetMathLibrary.MakeTransform` (+ (`SceneComponent.K2_GetComponentLocation` (`self.FloatingTextSpawnPoint`)) (* (`KismetMathLibrary.RandomUnitVector`) 20.0))) "AlwaysSpawn" "OverrideRootScale" null Text null))

(fn `TakeDamage`
  (params (DamageAmount :type "Float (double-precision)") (Dealer :type "Actor Object Reference"))
  (returns (IsDead :type Boolean))
  (bind _healthsys (`self.HealthSys`))
  (bind _out (`/Game/Dev_Content/Blueprints/Components/AC_HealthSystem.IsDead?` _healthsys))
  (`|ExecutionSequence`
    (:`then_0`
      (`/Game/Dev_Content/Blueprints/Components/AC_HealthSystem.SubtractHealth` (`self.HealthSys`) (`local.DamageAmount`))
      (`self.UpdateHealthUI` true)
      (`self.SpawnFloatingText` (`KismetTextLibrary.Conv_DoubleToText` (`local.DamageAmount`) "HalfToEven")))
    (:`then_1`
      (if _out
        (`self.OnDeath` (`local.Dealer`))))
    (:`then_2`
      (`/Engine/EditorBlueprintResources/StandardMacros.IsValid` _healthsys
        (:`Is Valid`
          (return _out))))))

(fn `Update_InputMode`
  (params (NewInputMode :type "/Game/UltimateMenu/Blueprints/Data/Enums/Enum_InputMode Enum" :default "NewEnumerator1"))
  (returns (Success :type Boolean))
  (return false))

(fn `Update_MenuType`
  (returns (Success :type Boolean))
  (return false))

(fn `UpdateHealthUI`
  (params (`Notify?` :type Boolean))
  (bind (_maxhealth _currenthealth) (`/Game/Dev_Content/Blueprints/Components/AC_HealthSystem.GetHealthStats` (`self.HealthSys`)))
  (bind _asui_status_bar_floating (cast `/Game/Dev_Content/Blueprints/UI/Status/UI_StatusBar_Floating` (`WidgetComponent.GetWidget` (`self.UI_StatusBar`))))
  (`/Game/Dev_Content/Blueprints/UI/Status/UI_StatusBar_Floating.UpdateHealth` _asui_status_bar_floating _maxhealth _currenthealth (`local.Notify?`)))

(fn `UpdateManaUI`
  (params (`Notify?` :type Boolean))
  (bind (_maxmana _currentmana) (`/Game/Dev_Content/Blueprints/Components/AC_ManaSystem.GetManaStats` (`self.ManaSys`)))
  (bind _asui_status_bar_floating (cast `/Game/Dev_Content/Blueprints/UI/Status/UI_StatusBar_Floating` (`WidgetComponent.GetWidget` (`self.UI_StatusBar`))))
  (`/Game/Dev_Content/Blueprints/UI/Status/UI_StatusBar_Floating.UpdateMana` _asui_status_bar_floating _maxmana _currentmana (`local.Notify?`)))

(fn `UseMana`
  (params (Amount :type "Float (double-precision)"))
  (`/Game/Dev_Content/Blueprints/Components/AC_ManaSystem.SubtractMana` (`self.ManaSys`) (`local.Amount`))
  (`self.UpdateManaUI` true)
  (return))

(fn `UserConstructionScript`)