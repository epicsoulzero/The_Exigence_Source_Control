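; BP_BasePet is a base pet actor that fights for its owner, with health, a floating status bar and status effects.
; OnAttack sphere-overlaps characters within attack range, excluding itself and its owner, dealing random damage scaled by the owner's level multiplier and credited to the owner.
; TakeDamage updates health and UI, spawns floating text and destroys the pet at death.
; Tick draws debug range circles; RespawnWithDelay is empty.
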(event `self.ReceiveBeginPlay`
  (`|ExecutionSequence`
    (:`then_0`
      (`self.K2_AddActorWorldOffset` (`KismetMathLibrary.MakeVector` 0.0 0.0 (`CapsuleComponent.GetScaledCapsuleHalfHeight` (`self.CapsuleComponent`))) false true))
    (:`then_1`
      (`self.UpdateHealthUI` false)
      (bind _asui_status_bar_floating (cast `/Game/Dev_Content/Blueprints/UI/Status/UI_StatusBar_Floating` (`WidgetComponent.GetWidget` (`self.UI_StatusBar`))))
      (`/Game/Dev_Content/Blueprints/UI/Status/UI_StatusBar_Floating.Initialize` _asui_status_bar_floating true false false))))

(event `self.ReceiveTick`
  (params (DeltaSeconds :type "Float (single-precision)"))
  (bind (_returnvalue_x _returnvalue_y) (`KismetMathLibrary.BreakVector` (`self.K2_GetActorLocation`)))
  (bind (_returnvalue_x_2 _returnvalue_y_2) (`KismetMathLibrary.BreakVector` (`self.K2_GetActorLocation`)))
  (`KismetSystemLibrary.DrawDebugCircle` (`KismetMathLibrary.MakeVector` _returnvalue_x_2 _returnvalue_y_2 10.0) (`self.AttackRange`) 50 (struct :`R` 1.0 :`A` 1.0) 0.0 2.0 (1.0 0.0 0.0) (0.0 1.0 0.0))
  (`KismetSystemLibrary.DrawDebugCircle` (`KismetMathLibrary.MakeVector` _returnvalue_x_2 _returnvalue_y_2 10.0) (`self.LookRange`) 50 (struct :`R` 1.0 :`G` 1.0 :`A` 1.0) 0.0 2.0 (1.0 0.0 0.0) (0.0 1.0 0.0))
  (`KismetSystemLibrary.DrawDebugCircle` (`KismetMathLibrary.MakeVector` _returnvalue_x _returnvalue_y 10.0) (`self.MaxRangeFromOwner`) 50 (struct :`B` 1.0 :`A` 1.0) 0.0 2.0 (1.0 0.0 0.0) (0.0 1.0 0.0)))

(event `/Game/Dev_Content/Blueprints/Interfaces/BPI_CanAttack.OnAttack`
  (params (TargetActor :type "Actor Object Reference"))
  (bind (_damagerange_x _damagerange_y) (`KismetMathLibrary.BreakVector2D` (`self.DamageRange`)))
  (bind (_outactors _returnvalue) (`KismetSystemLibrary.SphereOverlapActors` (`self.K2_GetActorLocation`) (`self.AttackRange`) (`|MakeArray` "ObjectTypeQuery1" "ObjectTypeQuery2" "ObjectTypeQuery3" :!type "EObjectTypeQuery Enum") "/Game/Dev_Content/Blueprints/Chars/BP_BaseCharacter.BP_BaseCharacter_C" (`|MakeArray` (`self.MyOwner`) self :!type "Actor Object Reference")))
  (if _returnvalue
    (for _array_element _outactors
      (message `/Game/Dev_Content/Blueprints/Interfaces/BPI_Damageable.TakeDamage` _array_element (`KismetMathLibrary.Conv_IntToDouble` (`KismetMathLibrary.Round` (* (`KismetMathLibrary.RandomFloatInRange` _damagerange_x _damagerange_y) (`/Game/Dev_Content/Blueprints/Chars/BP_BaseCharacter.GetLevelMultiplier` (cast `/Game/Dev_Content/Blueprints/Chars/Player/BP_PlayerCharacter` (`self.MyOwner`) :!pure true))))) (`self.MyOwner`)))))

(event `/Game/Dev_Content/Blueprints/Interfaces/BPI_StatusEffects.AddStatusEffect`
  (params (EffectToAdd :type "/Game/Dev_Content/Blueprints/Components/StatusEffects/AC_StatusEffect Object Reference"))
  (`/Game/Dev_Content/Blueprints/Components/StatusEffects/AC_StatusEffect_Manager.AddEffect` (`self.BPC_StatusEffect_Manager`) EffectToAdd))

(fn `RespawnWithDelay`
  (params (Owner :type "/Game/Dev_Content/Blueprints/Chars/Player/BP_PlayerCharacter Object Reference") (Delay :type "Float (double-precision)") (NewParam2 :type Boolean)))

(fn `SpawnFloatingText`
  (params (Text :type Text))
  (`|SpawnActorFromClass` "/Game/Dev_Content/Blueprints/Miscellaneous/BP_FloatingText.BP_FloatingText_C" (`KismetMathLibrary.MakeTransform` (+ (`SceneComponent.K2_GetComponentLocation` (`self.FloatingTextSpawnPoint`)) (* (`KismetMathLibrary.RandomUnitVector`) 50.0))) "AlwaysSpawn" "OverrideRootScale" null "" null))

(fn `TakeDamage`
  (params (DamageAmount :type "Float (double-precision)") (Dealer :type "Actor Object Reference"))
  (returns (IsDead :type Boolean))
  (`|ExecutionSequence`
    (:`then_0`
      (`/Game/Dev_Content/Blueprints/Components/AC_HealthSystem.SubtractHealth` (`self.HealthSys`) (`local.DamageAmount`))
      (`self.UpdateHealthUI` true)
      (`self.SpawnFloatingText` (`KismetTextLibrary.Conv_DoubleToText` (`local.DamageAmount`) "HalfToEven")))
    (:`then_1`
      (if (`/Game/Dev_Content/Blueprints/Components/AC_HealthSystem.IsDead?` (`self.HealthSys`))
        (`self.K2_DestroyActor`)
        (return true)
        (else
          (return false))))))

(fn `UpdateHealthUI`
  (params (`Notify?` :type Boolean))
  (bind (_maxhealth _currenthealth) (`/Game/Dev_Content/Blueprints/Components/AC_HealthSystem.GetHealthStats` (`self.HealthSys`)))
  (bind _asui_status_bar_floating (cast `/Game/Dev_Content/Blueprints/UI/Status/UI_StatusBar_Floating` (`WidgetComponent.GetWidget` (`self.UI_StatusBar`))))
  (`/Game/Dev_Content/Blueprints/UI/Status/UI_StatusBar_Floating.UpdateHealth` _asui_status_bar_floating _maxhealth _currenthealth (`local.Notify?`)))

(fn `UserConstructionScript`)