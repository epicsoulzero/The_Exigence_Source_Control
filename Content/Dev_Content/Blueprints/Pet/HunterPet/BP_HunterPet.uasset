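; BP_HunterPet is the hunter's pet character, with a charge attack that its BP_HunterPetController carries out.
; An init event starts the charge through the controller, and Tick ends it once the pet nears the charge location.
; A capsule overlap mid-charge deals sphere-overlap area damage credited to the owner, then ends the charge.
; Both endings add a brief movement-modifier status effect, with the overlap first clearing any active one.
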(event `self.ReceiveTick`
  (params (DeltaSeconds :type "Float (single-precision)"))
  (`parent.ReceiveTick` DeltaSeconds)
  (if (`self.IsCharging?`)
    (if (< (`KismetMathLibrary.Vector_Distance` (`self.K2_GetActorLocation`) (`self.ChargeLocation`)) (`self.MinDistToChargeLoc`))
      (set `self.IsCharging?` false)
      (bind _asbp_hunter_pet_controller (cast `/Game/Dev_Content/Blueprints/Pet/HunterPet/BP_HunterPetController` (`self.GetController`)))
      (`/Game/Dev_Content/Blueprints/Pet/HunterPet/BP_HunterPetController.EndChargeAbility` _asbp_hunter_pet_controller)
      (`|AddComponentByClass` "/Game/Dev_Content/Blueprints/Components/StatusEffects/AC_MovementModifier_SE.AC_MovementModifier_SE_C" 0.0 0.0 null 0.0 0.2))))

(event `Event_InitChargeSkill`
  (params (ChargeTarget :type "Actor Object Reference") (ChargeLocation :type "Vector Structure"))
  (if (not (`self.IsCharging?`))
    (bind _asbp_hunter_pet_controller (cast `/Game/Dev_Content/Blueprints/Pet/HunterPet/BP_HunterPetController` (`self.GetController`)))
    (`/Game/Dev_Content/Blueprints/Pet/HunterPet/BP_HunterPetController.UseChargeAbility` _asbp_hunter_pet_controller ChargeTarget ChargeLocation)
    (set `self.IsCharging?` true)))

(event `self.CapsuleComponent.OnComponentBeginOverlap`
  (params (OverlappedComponent :type "PrimitiveComponent Object Reference") (OtherActor :type "Actor Object Reference") (OtherComp :type "PrimitiveComponent Object Reference") (OtherBodyIndex :type Integer) (bFromSweep :type Boolean) (SweepResult :type "HitResult Structure (by ref)"))
  (if (`self.IsCharging?`)
    (`|ExecutionSequence`
      (:`then_0`
        (`self.AreaDamage`))
      (:`then_1`
        (`KismetSystemLibrary.PrintString` (`KismetSystemLibrary.GetDisplayName` OtherActor))
        (`/Game/Dev_Content/Blueprints/Components/StatusEffects/AC_StatusEffect_Manager.Early Exit By Class` (`self.BPC_StatusEffect_Manager`) "/Game/Dev_Content/Blueprints/Components/StatusEffects/AC_MovementModifier_SE.AC_MovementModifier_SE_C")
        (bind _asbp_hunter_pet_controller (cast `/Game/Dev_Content/Blueprints/Pet/HunterPet/BP_HunterPetController` (`self.GetController`)))
        (`/Game/Dev_Content/Blueprints/Pet/HunterPet/BP_HunterPetController.EndChargeAbility` _asbp_hunter_pet_controller)
        (`|AddComponentByClass` "/Game/Dev_Content/Blueprints/Components/StatusEffects/AC_MovementModifier_SE.AC_MovementModifier_SE_C" 0.0 0.0 null 0.0 0.2))
      (:`then_2`
        (set `self.IsCharging?` false)))))

(fn `AreaDamage`
  (bind _outactors (`KismetSystemLibrary.SphereOverlapActors` (`self.K2_GetActorLocation`) (`self.AttackRange`) (`|MakeArray` "ObjectTypeQuery11" :!type "EObjectTypeQuery Enum")))
  (for _array_element _outactors
    (message `/Game/Dev_Content/Blueprints/Interfaces/BPI_Damageable.TakeDamage` _array_element (`self.ChargeDamage`) (`self.MyOwner`))))

(fn `UserConstructionScript`
  (`parent.UserConstructionScript`))