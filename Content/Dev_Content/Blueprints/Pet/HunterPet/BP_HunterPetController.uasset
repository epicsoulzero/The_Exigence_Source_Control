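; AI controller for the hunter pet that drives its charge ability through Blackboard keys.
; On BeginPlay, after a short delay, it casts the pet reference to BP_HunterPet, caches it and writes its charge time to the Blackboard.
; UseChargeAbility sets the charge flag with either a valid target actor or a fallback location.
; EndChargeAbility resets the flag and clears both target keys.
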(event `self.ReceiveBeginPlay`
  (`parent.ReceiveBeginPlay`)
  (`KismetSystemLibrary.Delay` 0.1)
  (bind _asbp_hunter_pet (cast `/Game/Dev_Content/Blueprints/Pet/HunterPet/BP_HunterPet` (`self.Ref_Pet_BP`))
    (:`then`
      (set `self.Ref_HunterPet_BP` _asbp_hunter_pet)
      (`BlackboardComponent.SetValueAsFloat` (`AIBlueprintHelperLibrary.GetBlackboard` null) "ChargeTime" (`/Game/Dev_Content/Blueprints/Pet/HunterPet/BP_HunterPet.ChargeTime` (`self.Ref_HunterPet_BP`))))
    (:`CastFailed`
      (`KismetSystemLibrary.PrintString` "Cast failed"))))

(fn `EndChargeAbility`
  (`BlackboardComponent.SetValueAsBool` (`AIBlueprintHelperLibrary.GetBlackboard` null) "UseSkill_Charge" false)
  (`BlackboardComponent.ClearValue` (`AIBlueprintHelperLibrary.GetBlackboard` null) "ChargeTarget")
  (`BlackboardComponent.ClearValue` (`AIBlueprintHelperLibrary.GetBlackboard` null) "ChargeLocation"))

(fn `UseChargeAbility`
  (params (ChargeTarget :type "Actor Object Reference") (ChargeLocation :type "Vector Structure"))
  (`BlackboardComponent.SetValueAsBool` (`AIBlueprintHelperLibrary.GetBlackboard` null) "UseSkill_Charge" true)
  (`/Engine/EditorBlueprintResources/StandardMacros.IsValid` ChargeTarget
    (:`Is Valid`
      (`BlackboardComponent.SetValueAsObject` (`AIBlueprintHelperLibrary.GetBlackboard` null) "ChargeTarget" (`local.ChargeTarget`)))
    (:`Is Not Valid`
      (`BlackboardComponent.SetValueAsVector` (`AIBlueprintHelperLibrary.GetBlackboard` null) "ChargeLocation" (`local.ChargeLocation`)))))

(fn `UserConstructionScript`
  (`parent.UserConstructionScript`))