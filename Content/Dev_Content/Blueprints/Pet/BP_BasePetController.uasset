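; Base AI controller for pets that starts the pet's behavior tree.
; Shortly after BeginPlay, it casts the controlled pawn to BP_BasePet, caches it and runs the behavior tree that pet specifies.
; It then copies the pet's attack, look and leash ranges, attack speed and owner into the blackboard, so each pet supplies its own AI tuning.
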(event `self.ReceiveBeginPlay`
  (`KismetSystemLibrary.Delay` 0.1)
  (bind _asbp_base_pet (cast `/Game/Dev_Content/Blueprints/Pet/BP_BasePet` (`self.K2_GetPawn`)))
  (bind _output_get (set `self.Ref_Pet_BP` _asbp_base_pet))
  (`self.RunBehaviorTree` (`/Game/Dev_Content/Blueprints/Pet/BP_BasePet.BehaviorTreeRef` _output_get))
  (`BlackboardComponent.SetValueAsFloat` (`AIBlueprintHelperLibrary.GetBlackboard` null) "AttackRange" (`/Game/Dev_Content/Blueprints/Pet/BP_BasePet.AttackRange` (`self.Ref_Pet_BP`)))
  (`BlackboardComponent.SetValueAsFloat` (`AIBlueprintHelperLibrary.GetBlackboard` null) "AttackSpeed" (`/Game/Dev_Content/Blueprints/Pet/BP_BasePet.AttackSpeed` (`self.Ref_Pet_BP`)))
  (`BlackboardComponent.SetValueAsFloat` (`AIBlueprintHelperLibrary.GetBlackboard` null) "LookRange" (`/Game/Dev_Content/Blueprints/Pet/BP_BasePet.LookRange` (`self.Ref_Pet_BP`)))
  (`BlackboardComponent.SetValueAsFloat` (`AIBlueprintHelperLibrary.GetBlackboard` null) "MaxRangeFromOwner" (`/Game/Dev_Content/Blueprints/Pet/BP_BasePet.MaxRangeFromOwner` (`self.Ref_Pet_BP`)))
  (`BlackboardComponent.SetValueAsObject` (`AIBlueprintHelperLibrary.GetBlackboard` null) "OwnerActor" (`/Game/Dev_Content/Blueprints/Pet/BP_BasePet.MyOwner` (`self.Ref_Pet_BP`))))

(fn `UserConstructionScript`)