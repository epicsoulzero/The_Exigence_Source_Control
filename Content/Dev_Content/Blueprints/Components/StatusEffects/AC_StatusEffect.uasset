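; Base status effect component that registers with its owner through BPI_StatusEffects on BeginPlay.
; Trigger waits a delay, then starts a duration timer and calls ApplyEffect, an empty hook for child effects; Renew resets the timer and reapplies.
; When time runs out on Tick, OnExit removes it from the StatusEffectManager and schedules destruction.
; While not in effect, a separate countdown also destroys the component.
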(event `self.ReceiveBeginPlay`
  (if (`KismetSystemLibrary.DoesImplementInterface` (`self.GetOwner`) "/Game/Dev_Content/Blueprints/Interfaces/BPI_StatusEffects.BPI_StatusEffects_C")
    (message `/Game/Dev_Content/Blueprints/Interfaces/BPI_StatusEffects.AddStatusEffect` (`self.GetOwner`) self)))

(event `Trigger`
  (`KismetSystemLibrary.Delay` (`self.Delay`))
  (set `self.InternalTimer` (`self.Duration`))
  (set `self.InEffect?` true)
  (`self.ApplyEffect`))

(event `self.ReceiveTick`
  (params (DeltaSeconds :type "Float (single-precision)"))
  (set `self.DeltaTime` DeltaSeconds)
  (if (not (`self.IsBeingDestroyed`))
    (if (`self.InEffect?`)
      (bind _output_get (set `self.InternalTimer` (- (`self.InternalTimer`) (`self.DeltaTime`))))
      (if (<= _output_get 0.0)
        (`self.OnExit`))
      (else
        (bind _output_get_2 (set `self.DestroyTimer` (- (`self.DestroyTimer`) (`self.DeltaTime`))))
        (if (< _output_get_2 0.0)
          (`self.K2_DestroyComponent`))))))

(event `Event_DelayedDestroy`
  (params (Delay :type "Float (double-precision)"))
  (`KismetSystemLibrary.Delay` Delay)
  (`KismetSystemLibrary.PrintString` "Delayed destroy triggered" (`self.ShowDebugs`) false)
  (`self.K2_DestroyComponent`))

(fn `ApplyEffect`)

(fn `OnExit`
  (`/Engine/EditorBlueprintResources/StandardMacros.IsValid` (`self.GetOwner`)
    (:`Is Valid`
      (`/Engine/EditorBlueprintResources/StandardMacros.IsValid` (`self.StatusEffectManager`)
        (:`Is Valid`
          (`|ExecutionSequence`
            (:`then_0`
              (`/Game/Dev_Content/Blueprints/Components/StatusEffects/AC_StatusEffect_Manager.RemoveEffect` (`self.StatusEffectManager`) self))
            (:`then_1`
              (set `self.InEffect?` false)
              (`self.Event_DelayedDestroy` 0.1))
            (:`then_2`
              ;[1 1 1] Debugging
              (`KismetSystemLibrary.PrintString` (`KismetStringLibrary.Concat_StrStr` "Destroy Component: " (`KismetSystemLibrary.GetDisplayName` self)) (`self.ShowDebugs`) false (struct :`R` 1.0 :`G` 0.5 :`A` 1.0)))))))))

(fn `Renew`
  (set `self.InternalTimer` (`self.Duration`))
  (`self.ApplyEffect`))