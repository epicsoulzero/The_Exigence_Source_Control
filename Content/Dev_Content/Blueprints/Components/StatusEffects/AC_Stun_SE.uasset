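; Stun status effect component that stops its owner from accelerating while active.
; ApplyEffect runs only while no movement component is cached: it finds the owner's CharacterMovementComponent, saves its max acceleration, zeroes it and sends the owner a stun message.
; OnExit restores the saved acceleration, sends the owner the stun-ended message and then calls the parent exit logic.
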(fn `ApplyEffect`
  (`/Engine/EditorBlueprintResources/StandardMacros.IsValid` (`self.Ref_CharMovementComponent`)
    (:`Is Not Valid`
      (bind _output_get (set `self.Ref_CharMovementComponent` (`Actor.GetComponentByClass` (`self.GetOwner`) "/Script/Engine.CharacterMovementComponent")))
      (`/Engine/EditorBlueprintResources/StandardMacros.IsValid` _output_get
        (:`Is Valid`
          (set `self.Acceleration_Default` (`CharacterMovementComponent.GetMaxAcceleration` (`self.Ref_CharMovementComponent`)))
          (set `CharacterMovementComponent.MaxAcceleration` 0.0 (`self.Ref_CharMovementComponent`))
          (message `/Game/Dev_Content/Blueprints/Interfaces/BPI_StatusEffects.OnStun` (`self.GetOwner`) true))))))

(fn `OnExit`
  (bind _ref_charmovementcomponent (`self.Ref_CharMovementComponent`))
  (`|ExecutionSequence`
    (:`then_0`
      (`/Engine/EditorBlueprintResources/StandardMacros.IsValid` _ref_charmovementcomponent
        (:`Is Valid`
          (set `CharacterMovementComponent.MaxAcceleration` (`self.Acceleration_Default`) _ref_charmovementcomponent))))
    (:`then_1`
      (message `/Game/Dev_Content/Blueprints/Interfaces/BPI_StatusEffects.OnStun` (`self.GetOwner`) false))
    (:`then_2`
      (`parent.OnExit`))))