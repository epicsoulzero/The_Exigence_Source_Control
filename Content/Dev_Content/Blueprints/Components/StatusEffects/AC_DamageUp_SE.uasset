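; Status effect component that raises its owner's base damage multiplier for as long as the effect lasts.
; ApplyEffect finds and caches the owner's AC_StatsSystem, then passes Multiplier to ModifyBaseDamageMultiplier.
; OnExit sends the same Multiplier with the other modification type to undo the change, then runs the parent exit logic.
; BeginPlay and Tick are disabled stubs, so all behavior lives in these two overrides.
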(fn `ApplyEffect`
  (bind _output_get (set `self.Ref_StatsSystem` (`Actor.GetComponentByClass` (`self.GetOwner`) "/Game/Dev_Content/Blueprints/Components/AC_StatsSystem.AC_StatsSystem_C")))
  (`/Engine/EditorBlueprintResources/StandardMacros.IsValid` _output_get
    (:`Is Valid`
      (`/Game/Dev_Content/Blueprints/Components/AC_StatsSystem.ModifyBaseDamageMultiplier` (`self.Ref_StatsSystem`) (`self.Multiplier`) "NewEnumerator0"))))

(fn `OnExit`
  (`|ExecutionSequence`
    (:`then_0`
      (`/Engine/EditorBlueprintResources/StandardMacros.IsValid` (`self.Ref_StatsSystem`)
        (:`Is Valid`
          (`/Game/Dev_Content/Blueprints/Components/AC_StatsSystem.ModifyBaseDamageMultiplier` (`self.Ref_StatsSystem`) (`self.Multiplier`) "NewEnumerator1"))))
    (:`then_1`
      (`parent.OnExit`))))