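; Actor component that manages the status effects active on its owner.
; AddEffect looks for an active effect of the same class: stackable or new effects are triggered, stored and given a back-reference to the manager, while non-stackable duplicates renew the existing instance and are destroyed after a short delay.
; RemoveEffect drops a given instance from the list.
; EarlyExitByClass ends and removes the first active effect matching a class.
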(fn `AddEffect`
  (params (NewStatusEffect :type "/Game/Dev_Content/Blueprints/Components/StatusEffects/AC_StatusEffect Object Reference"))
  (locals (FirstInstance :type "/Game/Dev_Content/Blueprints/Components/StatusEffects/AC_StatusEffect Object Reference"))
  (bind _firstinstance (`local.FirstInstance`))
  (bind _newstatuseffect (`local.NewStatusEffect`))
  (bind _newstatuseffect_2 (`local.NewStatusEffect`))
  (bind _newstatuseffect_3 (`local.NewStatusEffect`))
  (`/Engine/EditorBlueprintResources/StandardMacros.IsValid` NewStatusEffect
    (:`Is Valid`
      (if (> (`KismetArrayLibrary.Array_Length` (`self.ActiveStatusEffects`)) 0)
        (for _array_element (`self.ActiveStatusEffects`)
          (if (== (`GameplayStatics.GetObjectClass` (`local.NewStatusEffect`)) (`GameplayStatics.GetObjectClass` _array_element))
            (set `local.FirstInstance` _array_element)
            (break)))
        (`/Engine/EditorBlueprintResources/StandardMacros.IsValid` (`local.FirstInstance`)
          (:`Is Valid`
            (if (`/Game/Dev_Content/Blueprints/Components/StatusEffects/AC_StatusEffect.Stackable?` (`local.FirstInstance`))
              ;[1 1 1] Accept new status effect and trigger, add to active status effects array
              (`/Game/Dev_Content/Blueprints/Components/StatusEffects/AC_StatusEffect.Trigger` _newstatuseffect_3)
              (`KismetSystemLibrary.PrintString` (`KismetStringLibrary.Concat_StrStr` "Added status effect (stackable): " (`self.GetSplitName` _newstatuseffect_3)) (`self.ShowDebugs`) false (struct :`R` 1.0 :`G` 0.5 :`A` 1.0))
              ;[1 1 1] Add to active status effects list and reference self to new status effect
              (`KismetArrayLibrary.Array_Add` (`self.ActiveStatusEffects`) _newstatuseffect :!label _label)
              (set `/Game/Dev_Content/Blueprints/Components/StatusEffects/AC_StatusEffect.StatusEffectManager` self _newstatuseffect)
              (else
                ;[1 1 1] Renew already existing component
                (if (not (`self.IsBeingDestroyed` _firstinstance))
                  (`/Game/Dev_Content/Blueprints/Components/StatusEffects/AC_StatusEffect.Renew` _firstinstance)
                  (`/Game/Dev_Content/Blueprints/Components/StatusEffects/AC_StatusEffect.Event_DelayedDestroy` (`local.NewStatusEffect`) 0.3)
                  (`KismetSystemLibrary.PrintString` (`KismetStringLibrary.Concat_StrStr` "Status effect renewed: " (`self.GetSplitName` _firstinstance)) (`self.ShowDebugs`) false (struct :`R` 1.0 :`G` 0.5 :`A` 1.0))
                  (else
                    (`KismetSystemLibrary.PrintString` "Upon adding status effect, renew failed and nothing was added" (`self.ShowDebugs`) false (struct :`R` 1.0 :`A` 1.0) 5.0))))))
          (:`Is Not Valid`
            ;[1 1 1] Accept and add new status effect and add to active status effect array
            (`/Game/Dev_Content/Blueprints/Components/StatusEffects/AC_StatusEffect.Trigger` _newstatuseffect_2 :!label _label_2)
            (`KismetSystemLibrary.PrintString` (`KismetStringLibrary.Concat_StrStr` "New Status Effect Added: " (`self.GetSplitName` _newstatuseffect_2)) (`self.ShowDebugs`) false (struct :`R` 1.0 :`G` 0.5 :`A` 1.0))
            (goto _label)))
        (else
          (`KismetSystemLibrary.PrintString` "Active list is: Empty" (`self.ShowDebugs`) false (struct :`R` 1.0 :`A` 1.0))
          (goto _label_2))))
    (:`Is Not Valid`
      (`KismetSystemLibrary.PrintString` (`KismetStringLibrary.Concat_StrStr` (`self.GetSplitName` NewStatusEffect) "is not valid") (`self.ShowDebugs`) false (struct :`R` 1.0 :`G` 1.0 :`A` 1.0)))))

(fn `Early Exit By Class`
  (params (`SE Class` :type "/Game/Dev_Content/Blueprints/Components/StatusEffects/AC_StatusEffect Class Reference"))
  (for _array_element (`self.ActiveStatusEffects`)
    (bind _returnvalue (`GameplayStatics.GetObjectClass` _array_element))
    (if (== (`local.SE Class`) _returnvalue)
      (`KismetSystemLibrary.PrintString` (`KismetSystemLibrary.GetClassDisplayName` _returnvalue))
      (`/Game/Dev_Content/Blueprints/Components/StatusEffects/AC_StatusEffect.OnExit` _array_element)
      (`self.RemoveEffect` _array_element)
      (break))))

(fn `GetSplitName`
  (params (Object :type "Object Object Reference"))
  (returns (Out :type String))
  (return (`.RightS` (`KismetStringLibrary.Split` (`KismetSystemLibrary.GetDisplayName` Object) "." "IgnoreCase" "FromEnd"))))

(fn `RemoveEffect`
  (params (EffectToRemove :type "/Game/Dev_Content/Blueprints/Components/StatusEffects/AC_StatusEffect Object Reference"))
  (locals (IndexFound :type Integer))
  (bind _output_get (set `local.IndexFound` (`KismetArrayLibrary.Array_Find` (`self.ActiveStatusEffects`) EffectToRemove)))
  (if (!= _output_get -1)
    (`KismetArrayLibrary.Array_Remove` (`self.ActiveStatusEffects`) (`local.IndexFound`))
    (`KismetSystemLibrary.PrintString` "Status effect removed" true true (struct :`R` 1.0 :`G` 1.0 :`A` 1.0))
    (else
      (`KismetSystemLibrary.PrintString` "Effect not found"))))