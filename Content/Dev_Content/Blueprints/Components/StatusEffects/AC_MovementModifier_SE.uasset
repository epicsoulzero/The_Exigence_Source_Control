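; Status effect component that modifies its owner's movement speed while active, working through the owner's AC_MoveSpeedManager.
; On BeginPlay it finds the manager and caches the current main multiplier.
; ApplyEffect sets the effect's main multiplier and modifies the additive one, with an optional debug print.
; OnExit restores the cached multiplier, modifies the additive one in another mode, and calls the parent exit only if the manager is valid.
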(event `self.ReceiveBeginPlay`
  (`self.GetDefaultValues`)
  (`parent.ReceiveBeginPlay`))

(fn `ApplyEffect`
  (`/Engine/EditorBlueprintResources/StandardMacros.IsValid` (`self.MoveSpeedManager`)
    (:`Is Valid`
      (`/Game/Dev_Content/Blueprints/Components/AC_MoveSpeedManager.SetMainMultiplier` (`self.MoveSpeedManager`) (`self.MainMult_Effect`))
      (`/Game/Dev_Content/Blueprints/Components/AC_MoveSpeedManager.ModifyAdditiveMultiplier` (`self.MoveSpeedManager`) (`self.AdditiveMult_Effect`) "NewEnumerator0")
      (`KismetSystemLibrary.PrintString` "Walk Speed has been reduced to 0" (`self.ShowDebugs`) false (struct :`G` 0.5 :`B` 1.0 :`A` 1.0)))))

(fn `GetDefaultValues`
  (bind _output_get (set `self.MoveSpeedManager` (`Actor.GetComponentByClass` (`self.GetOwner`) "/Game/Dev_Content/Blueprints/Components/AC_MoveSpeedManager.AC_MoveSpeedManager_C")))
  (`/Engine/EditorBlueprintResources/StandardMacros.IsValid` _output_get
    (:`Is Valid`
      (set `self.Multiplier_Actual` (`/Game/Dev_Content/Blueprints/Components/AC_MoveSpeedManager.Multiplier_Main` (`self.MoveSpeedManager`))))))

(fn `OnExit`
  (`/Engine/EditorBlueprintResources/StandardMacros.IsValid` (`self.MoveSpeedManager`)
    (:`Is Valid`
      (`/Game/Dev_Content/Blueprints/Components/AC_MoveSpeedManager.SetMainMultiplier` (`self.MoveSpeedManager`) (`self.Multiplier_Actual`))
      (`/Game/Dev_Content/Blueprints/Components/AC_MoveSpeedManager.ModifyAdditiveMultiplier` (`self.MoveSpeedManager`) (`self.AdditiveMult_Effect`) "NewEnumerator1")
      (`parent.OnExit`))))