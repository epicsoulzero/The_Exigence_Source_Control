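; Mana component that tracks current and maximum mana and regenerates it at a flat rate each Tick while below the maximum.
; Add, subtract and max-mana changes that refill route through one clamped setter, which fires the current-mana-changed notification.
; It also exposes a stats getter and an affordability check for spending mana.
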(event `self.ReceiveTick`
  (params (DeltaSeconds :type "Float (single-precision)"))
  (if (< (`self.CurrentMana`) (`self.MaxMana`))
    (`self.AddMana` (* (`self.FlatRegenRate`) DeltaSeconds))))

(fn `AddMana`
  (params (Amount :type "Float (double-precision)"))
  (`self.SetCurrentManaClamped` (+ Amount (`self.CurrentMana`))))

(fn `GetManaStats`
  (returns (MaxMana :type "Float (double-precision)") (CurrentMana :type "Float (double-precision)"))
  (return (`self.MaxMana`) (`self.CurrentMana`)))

(fn `HasEnoughMana?`
  (params (Amount :type "Float (double-precision)"))
  (returns (Out :type Boolean))
  (return (<= Amount (`self.CurrentMana`))))

(fn `SetCurrentManaClamped`
  (params (NewValue :type "Float (double-precision)"))
  (set `self.CurrentMana` (`KismetMathLibrary.FClamp` NewValue 0.0 (`self.MaxMana`)))
  (`self.OnCurrentManaChanged`))

(fn `SetMaxMana`
  (params (NewMax :type "Float (double-precision)") (`SetCurrentToMax?` :type Boolean :default true))
  (bind _output_get (set `self.MaxMana` NewMax))
  (if `SetCurrentToMax?`
    (`self.SetCurrentManaClamped` _output_get)))

(fn `SubtractMana`
  (params (Amount :type "Float (double-precision)"))
  (`self.SetCurrentManaClamped` (- (`self.CurrentMana`) Amount)))