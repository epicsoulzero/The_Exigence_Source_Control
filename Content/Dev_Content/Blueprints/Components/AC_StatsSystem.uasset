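; Actor component that holds a character's RPG stats as base and additive layers for primary stats and substats, loaded from data tables on BeginPlay.
; Strength, Agility and Intellect changes cascade through per-point modifiers into damage, health, attack speed, crit chance and energy.
; Getters sum both layers, with damage also scaled by a multiplier.
; Spell and elemental damage modifiers are empty stubs, and GetManaAmount's energy calculation is left unconnected.
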(event `self.ReceiveBeginPlay`
  (`self.InitializeStats`))

(fn `AppendAndConvertToName`
  (params (RowName :type String))
  (returns (Out :type Name))
  (return (`KismetStringLibrary.Conv_StringToName` (`KismetStringLibrary.Concat_StrStr` (`self.RowName`) RowName))))

(fn `GetArmor`
  (returns (Out :type Integer))
  (return (+ (`.Armor_11_2A0AF25049D7AF867E88D6B8416C5BD9` (break `/Game/Dev_Content/Structs/S_SubStats_Defensive` (`.Defensive_10_61502738442807B468EBCA8F9BA2D701` (break `/Game/Dev_Content/Structs/S_SubStats_All` (`self.SubStats_Base`))))) (`.Armor_11_2A0AF25049D7AF867E88D6B8416C5BD9` (break `/Game/Dev_Content/Structs/S_SubStats_Defensive` (`.Defensive_10_61502738442807B468EBCA8F9BA2D701` (break `/Game/Dev_Content/Structs/S_SubStats_All` (`self.SubStats_Additive`))))))))

(fn `GetArmorPenetration`
  (returns (Out :type Integer))
  (return (+ (`.ArmorPenetration_23_615731AA4D497932066FA6AF44EA7A8D` (break `/Game/Dev_Content/Structs/S_SubStats_Offensive` (`.Offensive_9_D88559E34BB9C3BDFF9365BCC90D44E4` (break `/Game/Dev_Content/Structs/S_SubStats_All` (`self.SubStats_Base`))))) (`.ArmorPenetration_23_615731AA4D497932066FA6AF44EA7A8D` (break `/Game/Dev_Content/Structs/S_SubStats_Offensive` (`.Offensive_9_D88559E34BB9C3BDFF9365BCC90D44E4` (break `/Game/Dev_Content/Structs/S_SubStats_All` (`self.SubStats_Additive`))))))))

(fn `GetAttackSpeed`
  (returns (Out :type "Float (double-precision)"))
  (return (+ (`.AttackSpeed_20_D955449940783FF68AF987B5DCDFFAF7` (break `/Game/Dev_Content/Structs/S_SubStats_Offensive` (`.Offensive_9_D88559E34BB9C3BDFF9365BCC90D44E4` (break `/Game/Dev_Content/Structs/S_SubStats_All` (`self.SubStats_Base`))))) (`.AttackSpeed_20_D955449940783FF68AF987B5DCDFFAF7` (break `/Game/Dev_Content/Structs/S_SubStats_Offensive` (`.Offensive_9_D88559E34BB9C3BDFF9365BCC90D44E4` (break `/Game/Dev_Content/Structs/S_SubStats_All` (`self.SubStats_Additive`))))))))

(fn `GetBlockChance`
  (returns (Out :type "Float (double-precision)"))
  (return (+ (`.BlockChance_14_E746DBB945544186CD373C95F344B9FE` (break `/Game/Dev_Content/Structs/S_SubStats_Defensive` (`.Defensive_10_61502738442807B468EBCA8F9BA2D701` (break `/Game/Dev_Content/Structs/S_SubStats_All` (`self.SubStats_Base`))))) (`.BlockChance_14_E746DBB945544186CD373C95F344B9FE` (break `/Game/Dev_Content/Structs/S_SubStats_Defensive` (`.Defensive_10_61502738442807B468EBCA8F9BA2D701` (break `/Game/Dev_Content/Structs/S_SubStats_All` (`self.SubStats_Additive`))))))))

(fn `GetCooldownReduction`
  (returns (Out :type "Float (double-precision)"))
  (return (+ (`.CooldownReduction_24_9BC36AE947466F556913349966625B7C` (break `/Game/Dev_Content/Structs/S_SubStats_Offensive` (`.Offensive_9_D88559E34BB9C3BDFF9365BCC90D44E4` (break `/Game/Dev_Content/Structs/S_SubStats_All` (`self.SubStats_Base`))))) (`.CooldownReduction_24_9BC36AE947466F556913349966625B7C` (break `/Game/Dev_Content/Structs/S_SubStats_Offensive` (`.Offensive_9_D88559E34BB9C3BDFF9365BCC90D44E4` (break `/Game/Dev_Content/Structs/S_SubStats_All` (`self.SubStats_Additive`))))))))

(fn `GetCritChance`
  (returns (Out :type "Float (double-precision)"))
  (return (+ (`.CriticalChance_27_13BD6E7B4853C1D64214229860612933` (break `/Game/Dev_Content/Structs/S_SubStats_Offensive` (`.Offensive_9_D88559E34BB9C3BDFF9365BCC90D44E4` (break `/Game/Dev_Content/Structs/S_SubStats_All` (`self.SubStats_Base`))))) (`.CriticalChance_27_13BD6E7B4853C1D64214229860612933` (break `/Game/Dev_Content/Structs/S_SubStats_Offensive` (`.Offensive_9_D88559E34BB9C3BDFF9365BCC90D44E4` (break `/Game/Dev_Content/Structs/S_SubStats_All` (`self.SubStats_Additive`))))))))

(fn `GetCritDamage`
  (returns (Out :type "Float (double-precision)"))
  (return (+ (`.CriticalDamage_42_96E8D0EC483ECEA1EEB5EFADBEA5D967` (break `/Game/Dev_Content/Structs/S_SubStats_Offensive` (`.Offensive_9_D88559E34BB9C3BDFF9365BCC90D44E4` (break `/Game/Dev_Content/Structs/S_SubStats_All` (`self.SubStats_Base`))))) (`.CriticalDamage_42_96E8D0EC483ECEA1EEB5EFADBEA5D967` (break `/Game/Dev_Content/Structs/S_SubStats_Offensive` (`.Offensive_9_D88559E34BB9C3BDFF9365BCC90D44E4` (break `/Game/Dev_Content/Structs/S_SubStats_All` (`self.SubStats_Additive`))))))))

(fn `GetDamage`
  (returns (MinDamage :type Integer) (MaxDamage :type Integer))
  (bind ((`BaseAttackDamage_Min_29_4E0461DD4A53AE0F8637378B561D89A4` _baseattackdamage_min) (`BaseAttackDamage_Max_30_527B76E540F80C7F4FC7E4898C7C70F0` _baseattackdamage_max) (`CriticalDamage_42_96E8D0EC483ECEA1EEB5EFADBEA5D967` _criticaldamage) (`BaseAttackDmgMult_41_F4E219434D7DCBF82BBDA4AF5C32AEDF` _baseattackdmgmult)) (break `/Game/Dev_Content/Structs/S_SubStats_Offensive` (`.Offensive_9_D88559E34BB9C3BDFF9365BCC90D44E4` (break `/Game/Dev_Content/Structs/S_SubStats_All` (`self.SubStats_Additive`)))))
  (bind ((`BaseAttackDamage_Min_29_4E0461DD4A53AE0F8637378B561D89A4` _baseattackdamage_min_2) (`BaseAttackDamage_Max_30_527B76E540F80C7F4FC7E4898C7C70F0` _baseattackdamage_max_2) (`CriticalDamage_42_96E8D0EC483ECEA1EEB5EFADBEA5D967` _criticaldamage_2) (`BaseAttackDmgMult_41_F4E219434D7DCBF82BBDA4AF5C32AEDF` _baseattackdmgmult_2)) (break `/Game/Dev_Content/Structs/S_SubStats_Offensive` (`.Offensive_9_D88559E34BB9C3BDFF9365BCC90D44E4` (break `/Game/Dev_Content/Structs/S_SubStats_All` (`self.SubStats_Base`)))))
  (bind _returnvalue (+ _baseattackdmgmult_2 _baseattackdmgmult))
  (return (`KismetMathLibrary.Round` (* (+ _baseattackdamage_min_2 _baseattackdamage_min) _returnvalue)) (`KismetMathLibrary.Round` (* (+ _baseattackdamage_max_2 _baseattackdamage_max) _returnvalue))))

(fn `GetDamageReduction`
  (returns (Out :type "Float (double-precision)"))
  (return (+ (`.DamageReduction_35_7CE2E0B24A2CDA0C5E0E719257526966` (break `/Game/Dev_Content/Structs/S_SubStats_Defensive` (`.Defensive_10_61502738442807B468EBCA8F9BA2D701` (break `/Game/Dev_Content/Structs/S_SubStats_All` (`self.SubStats_Base`))))) (`.DamageReduction_35_7CE2E0B24A2CDA0C5E0E719257526966` (break `/Game/Dev_Content/Structs/S_SubStats_Defensive` (`.Defensive_10_61502738442807B468EBCA8F9BA2D701` (break `/Game/Dev_Content/Structs/S_SubStats_All` (`self.SubStats_Additive`))))))))

(fn `GetEnergy`
  (returns (Out :type Integer))
  (return (+ (`.MaxEnergy_31_3BF29F7D497C1C0505D8FE857D2DA1ED` (break `/Game/Dev_Content/Structs/S_SubStats_Defensive` (`.Defensive_10_61502738442807B468EBCA8F9BA2D701` (break `/Game/Dev_Content/Structs/S_SubStats_All` (`self.SubStats_Base`))))) (`.MaxEnergy_31_3BF29F7D497C1C0505D8FE857D2DA1ED` (break `/Game/Dev_Content/Structs/S_SubStats_Defensive` (`.Defensive_10_61502738442807B468EBCA8F9BA2D701` (break `/Game/Dev_Content/Structs/S_SubStats_All` (`self.SubStats_Additive`))))))))

(fn `GetEnergyRegen`
  (returns (Out :type "Float (double-precision)"))
  (return (+ (`.EnergyRegen_32_5677FE0D4BEA8335AC9CE88EC1E1C0A9` (break `/Game/Dev_Content/Structs/S_SubStats_Defensive` (`.Defensive_10_61502738442807B468EBCA8F9BA2D701` (break `/Game/Dev_Content/Structs/S_SubStats_All` (`self.SubStats_Base`))))) (`.EnergyRegen_32_5677FE0D4BEA8335AC9CE88EC1E1C0A9` (break `/Game/Dev_Content/Structs/S_SubStats_Defensive` (`.Defensive_10_61502738442807B468EBCA8F9BA2D701` (break `/Game/Dev_Content/Structs/S_SubStats_All` (`self.SubStats_Additive`))))))))

(fn `GetEvasion`
  (returns (Out :type "Float (double-precision)"))
  (return (+ (`.Evasion_16_29BF514647FACB8CFD823DA117B4A060` (break `/Game/Dev_Content/Structs/S_SubStats_Defensive` (`.Defensive_10_61502738442807B468EBCA8F9BA2D701` (break `/Game/Dev_Content/Structs/S_SubStats_All` (`self.SubStats_Base`))))) (`.Evasion_16_29BF514647FACB8CFD823DA117B4A060` (break `/Game/Dev_Content/Structs/S_SubStats_Defensive` (`.Defensive_10_61502738442807B468EBCA8F9BA2D701` (break `/Game/Dev_Content/Structs/S_SubStats_All` (`self.SubStats_Additive`))))))))

(fn `GetHealth`
  (returns (Out :type Integer))
  (return (+ (`.MaxHealth_6_A72FEEB1411FA52892BB53952A4F1E3E` (break `/Game/Dev_Content/Structs/S_SubStats_Defensive` (`.Defensive_10_61502738442807B468EBCA8F9BA2D701` (break `/Game/Dev_Content/Structs/S_SubStats_All` (`self.SubStats_Base`))))) (`.MaxHealth_6_A72FEEB1411FA52892BB53952A4F1E3E` (break `/Game/Dev_Content/Structs/S_SubStats_Defensive` (`.Defensive_10_61502738442807B468EBCA8F9BA2D701` (break `/Game/Dev_Content/Structs/S_SubStats_All` (`self.SubStats_Additive`))))))))

(fn `GetHealthRegen`
  (returns (Out :type "Float (double-precision)"))
  (return (+ (`.HealthRegen_8_6E82B10C46F0D657528647ADCCDE2289` (break `/Game/Dev_Content/Structs/S_SubStats_Defensive` (`.Defensive_10_61502738442807B468EBCA8F9BA2D701` (break `/Game/Dev_Content/Structs/S_SubStats_All` (`self.SubStats_Base`))))) (`.HealthRegen_8_6E82B10C46F0D657528647ADCCDE2289` (break `/Game/Dev_Content/Structs/S_SubStats_Defensive` (`.Defensive_10_61502738442807B468EBCA8F9BA2D701` (break `/Game/Dev_Content/Structs/S_SubStats_All` (`self.SubStats_Additive`))))))))

(fn `GetLifeOnKill`
  (returns (Out :type Integer))
  (return (+ (`.LifeOnKill_23_26A9F6C04E206A4CE43C68AD7962913E` (break `/Game/Dev_Content/Structs/S_SubStats_Defensive` (`.Defensive_10_61502738442807B468EBCA8F9BA2D701` (break `/Game/Dev_Content/Structs/S_SubStats_All` (`self.SubStats_Base`))))) (`.LifeOnKill_23_26A9F6C04E206A4CE43C68AD7962913E` (break `/Game/Dev_Content/Structs/S_SubStats_Defensive` (`.Defensive_10_61502738442807B468EBCA8F9BA2D701` (break `/Game/Dev_Content/Structs/S_SubStats_All` (`self.SubStats_Additive`))))))))

(fn `GetLifesteal`
  (returns (Out :type "Float (double-precision)"))
  (return (+ (`.Lifesteal_18_11D39451420BFB007D7F29BDBE5135DD` (break `/Game/Dev_Content/Structs/S_SubStats_Defensive` (`.Defensive_10_61502738442807B468EBCA8F9BA2D701` (break `/Game/Dev_Content/Structs/S_SubStats_All` (`self.SubStats_Base`))))) (`.Lifesteal_18_11D39451420BFB007D7F29BDBE5135DD` (break `/Game/Dev_Content/Structs/S_SubStats_Defensive` (`.Defensive_10_61502738442807B468EBCA8F9BA2D701` (break `/Game/Dev_Content/Structs/S_SubStats_All` (`self.SubStats_Additive`))))))))

(fn `GetMovementSpeed`
  (returns (Out :type "Float (double-precision)"))
  (return (+ (`.MovementSpeed_22_C6D6D8B1402B48DACA9C619ED22A40BE` (break `/Game/Dev_Content/Structs/S_SubStats_Defensive` (`.Defensive_10_61502738442807B468EBCA8F9BA2D701` (break `/Game/Dev_Content/Structs/S_SubStats_All` (`self.SubStats_Base`))))) (`.MovementSpeed_22_C6D6D8B1402B48DACA9C619ED22A40BE` (break `/Game/Dev_Content/Structs/S_SubStats_Defensive` (`.Defensive_10_61502738442807B468EBCA8F9BA2D701` (break `/Game/Dev_Content/Structs/S_SubStats_All` (`self.SubStats_Additive`))))))))

(fn `GetPrimaryStats`
  (returns (Strength :type Integer) (Agility :type Integer) (Intellect :type Integer))
  (bind (_strength _agility _intellect) (break `/Game/Dev_Content/Structs/S_PrimaryStats` (`self.Primary_Additive`)))
  (bind (_strength_2 _agility_2 _intellect_2) (break `/Game/Dev_Content/Structs/S_PrimaryStats` (`self.Primary_Base`)))
  (return (+ _strength_2 _strength) (+ _agility_2 _agility) (+ _intellect_2 _intellect)))

(fn `GetResists`
  (returns (Resists :type "/Game/Dev_Content/Structs/S_SubStats_Resists Structure"))
  (bind (_physical _bleed _poison _cold _fire _lightning _holy _hell) (break `/Game/Dev_Content/Structs/S_SubStats_Resists` (`.Resists_11_AA18666D49DA076EA370EF94E0DFF173` (break `/Game/Dev_Content/Structs/S_SubStats_All` (`self.SubStats_Base`)))))
  (bind (_physical_2 _bleed_2 _poison_2 _cold_2 _fire_2 _lightning_2 _holy_2 _hell_2) (break `/Game/Dev_Content/Structs/S_SubStats_Resists` (`.Resists_11_AA18666D49DA076EA370EF94E0DFF173` (break `/Game/Dev_Content/Structs/S_SubStats_All` (`self.SubStats_Additive`)))))
  (return (make `/Game/Dev_Content/Structs/S_SubStats_Resists` (+ _physical _physical_2) (+ _bleed _bleed_2) (+ _poison _poison_2) (+ _cold _cold_2) (+ _fire _fire_2) (+ _lightning _lightning_2) (+ _holy _holy_2) (+ _hell _hell_2))))

(fn `InitializeStats`
  (`|ExecutionSequence`
    (:`then_0`
      ;[1 1 1] Get and set base and additive primary stats
      (`|ExecutionSequence`
        (:`then_0`
          (bind _returnvalue (`|GetDataTableRow` "/Game/Dev_Content/DataTables/DT_PrimaryStats.DT_PrimaryStats" (`self.AppendAndConvertToName` "_Base"))
            (:`then`
              (set `self.Primary_Base` _returnvalue))))
        (:`then_1`
          (bind _returnvalue_2 (`|GetDataTableRow` "/Game/Dev_Content/DataTables/DT_PrimaryStats.DT_PrimaryStats" (`self.AppendAndConvertToName` "_Additive"))
            (:`then`
              (set `self.Primary_Additive` _returnvalue_2))))))
    (:`then_1`
      ;[1 1 1] Get and set base and additive substats
      (`|ExecutionSequence`
        (:`then_0`
          (bind _returnvalue_3 (`|GetDataTableRow` "/Game/Dev_Content/DataTables/DT_Stats_All.DT_Stats_All" (`self.AppendAndConvertToName` "_Base"))
            (:`then`
              (set `self.SubStats_Base` _returnvalue_3))))
        (:`then_1`
          (bind _returnvalue_4 (`|GetDataTableRow` "/Game/Dev_Content/DataTables/DT_Stats_All.DT_Stats_All" (`self.AppendAndConvertToName` "_Additive"))
            (:`then`
              (set `self.SubStats_Additive` _returnvalue_4))))))
    (:`then_2`
      ;[1 1 1] Get substat modifiers
      (bind _returnvalue_5 (`|GetDataTableRow` "/Game/Dev_Content/DataTables/DT_Substats_Modifiers.DT_Substats_Modifiers" (`KismetStringLibrary.Conv_StringToName` (`self.RowName`)))
        (:`then`
          (set `self.Substats_Modifiers` _returnvalue_5))))))

(fn `ModifiyEnergy`
  (params (Amount :type Integer) (ModType :type "/Game/Dev_Content/Enums/E_ModType Enum" :default "NewEnumerator0"))
  (switch `/Game/Dev_Content/Enums/E_ModType` ModType
    (:`NewEnumerator0`
      (setmembers `/Game/Dev_Content/Structs/S_SubStats_Defensive` :`StructRef` (`.Defensive_10_61502738442807B468EBCA8F9BA2D701` (break `/Game/Dev_Content/Structs/S_SubStats_All` (`self.SubStats_Additive`))) :`MaxEnergy` (+ (`.MaxEnergy_31_3BF29F7D497C1C0505D8FE857D2DA1ED` (break `/Game/Dev_Content/Structs/S_SubStats_Defensive` (`.Defensive_10_61502738442807B468EBCA8F9BA2D701` (break `/Game/Dev_Content/Structs/S_SubStats_All` (`self.SubStats_Additive`))))) (`local.Amount`))))
    (:`NewEnumerator1`
      (setmembers `/Game/Dev_Content/Structs/S_SubStats_Defensive` :`StructRef` (`.Defensive_10_61502738442807B468EBCA8F9BA2D701` (break `/Game/Dev_Content/Structs/S_SubStats_All` (`self.SubStats_Additive`))) :`MaxEnergy` (- (`.MaxEnergy_31_3BF29F7D497C1C0505D8FE857D2DA1ED` (break `/Game/Dev_Content/Structs/S_SubStats_Defensive` (`.Defensive_10_61502738442807B468EBCA8F9BA2D701` (break `/Game/Dev_Content/Structs/S_SubStats_All` (`self.SubStats_Additive`))))) (`local.Amount`))))))

(fn `ModifyAgility`
  (params (Amount :type Integer) (ModType :type "/Game/Dev_Content/Enums/E_ModType Enum" :default "NewEnumerator0"))
  (`|ExecutionSequence`
    (:`then_0`
      (switch `/Game/Dev_Content/Enums/E_ModType` (`local.ModType`)
        (:`NewEnumerator0`
          (setmembers `/Game/Dev_Content/Structs/S_PrimaryStats` :`StructRef` (`self.Primary_Additive`) :`Agility` (+ (`.Agility_4_04AC057146971CE95276F4BEEDA43EB3` (break `/Game/Dev_Content/Structs/S_PrimaryStats` (`self.Primary_Additive`))) (`local.Amount`))))
        (:`NewEnumerator1`
          (setmembers `/Game/Dev_Content/Structs/S_PrimaryStats` :`StructRef` (`self.Primary_Additive`) :`Agility` (- (`.Agility_4_04AC057146971CE95276F4BEEDA43EB3` (break `/Game/Dev_Content/Structs/S_PrimaryStats` (`self.Primary_Additive`))) (`local.Amount`))))))
    (:`then_1`
      (`self.ModifyAttackSpeed` (* (`.AttackSpeed_20_D955449940783FF68AF987B5DCDFFAF7` (break `/Game/Dev_Content/Structs/S_SubStats_Offensive` (`.Offensive_9_D88559E34BB9C3BDFF9365BCC90D44E4` (break `/Game/Dev_Content/Structs/S_SubStats_All` (`self.Substats_Modifiers`))))) (`local.Amount`)) (`local.ModType`)))
    (:`then_2`
      (`self.ModifyCriticalChance` (* (`.CriticalChance_27_13BD6E7B4853C1D64214229860612933` (break `/Game/Dev_Content/Structs/S_SubStats_Offensive` (`.Offensive_9_D88559E34BB9C3BDFF9365BCC90D44E4` (break `/Game/Dev_Content/Structs/S_SubStats_All` (`self.Substats_Modifiers`))))) (`local.Amount`)) (`local.ModType`)))))

(fn `ModifyAttackDamage`
  (params (Amount_Min :type Integer) (Amount_Max :type Integer) (ModType :type "/Game/Dev_Content/Enums/E_ModType Enum" :default "NewEnumerator0"))
  (bind ((`BaseAttackDamage_Min_29_4E0461DD4A53AE0F8637378B561D89A4` _baseattackdamage_min) (`BaseAttackDamage_Max_30_527B76E540F80C7F4FC7E4898C7C70F0` _baseattackdamage_max)) (break `/Game/Dev_Content/Structs/S_SubStats_Offensive` (`.Offensive_9_D88559E34BB9C3BDFF9365BCC90D44E4` (break `/Game/Dev_Content/Structs/S_SubStats_All` (`self.SubStats_Additive`)))))
  (bind ((`BaseAttackDamage_Min_29_4E0461DD4A53AE0F8637378B561D89A4` _baseattackdamage_min_2) (`BaseAttackDamage_Max_30_527B76E540F80C7F4FC7E4898C7C70F0` _baseattackdamage_max_2)) (break `/Game/Dev_Content/Structs/S_SubStats_Offensive` (`.Offensive_9_D88559E34BB9C3BDFF9365BCC90D44E4` (break `/Game/Dev_Content/Structs/S_SubStats_All` (`self.SubStats_Additive`)))))
  (switch `/Game/Dev_Content/Enums/E_ModType` ModType
    (:`NewEnumerator0`
      (setmembers `/Game/Dev_Content/Structs/S_SubStats_Offensive` :`StructRef` (`.Offensive_9_D88559E34BB9C3BDFF9365BCC90D44E4` (break `/Game/Dev_Content/Structs/S_SubStats_All` (`self.SubStats_Additive`))) :`BaseAttackDamage_Min` (+ _baseattackdamage_min_2 (`local.Amount_Min`)) :`BaseAttackDamage_Max` (+ _baseattackdamage_max_2 (`local.Amount_Max`))))
    (:`NewEnumerator1`
      (setmembers `/Game/Dev_Content/Structs/S_SubStats_Offensive` :`StructRef` (`.Offensive_9_D88559E34BB9C3BDFF9365BCC90D44E4` (break `/Game/Dev_Content/Structs/S_SubStats_All` (`self.SubStats_Additive`))) :`BaseAttackDamage_Min` (- _baseattackdamage_min (`local.Amount_Min`)) :`BaseAttackDamage_Max` (- _baseattackdamage_max (`local.Amount_Max`))))))

(fn `ModifyAttackSpeed`
  (params (Amount :type "Float (double-precision)") (ModType :type "/Game/Dev_Content/Enums/E_ModType Enum" :default "NewEnumerator0"))
  (switch `/Game/Dev_Content/Enums/E_ModType` ModType
    (:`NewEnumerator0`
      (setmembers `/Game/Dev_Content/Structs/S_SubStats_Offensive` :`StructRef` (`.Offensive_9_D88559E34BB9C3BDFF9365BCC90D44E4` (break `/Game/Dev_Content/Structs/S_SubStats_All` (`self.SubStats_Additive`))) :`AttackSpeed` (+ (`.AttackSpeed_20_D955449940783FF68AF987B5DCDFFAF7` (break `/Game/Dev_Content/Structs/S_SubStats_Offensive` (`.Offensive_9_D88559E34BB9C3BDFF9365BCC90D44E4` (break `/Game/Dev_Content/Structs/S_SubStats_All` (`self.SubStats_Additive`))))) (`local.Amount`))))
    (:`NewEnumerator1`
      (setmembers `/Game/Dev_Content/Structs/S_SubStats_Offensive` :`StructRef` (`.Offensive_9_D88559E34BB9C3BDFF9365BCC90D44E4` (break `/Game/Dev_Content/Structs/S_SubStats_All` (`self.SubStats_Additive`))) :`AttackSpeed` (- (`.AttackSpeed_20_D955449940783FF68AF987B5DCDFFAF7` (break `/Game/Dev_Content/Structs/S_SubStats_Offensive` (`.Offensive_9_D88559E34BB9C3BDFF9365BCC90D44E4` (break `/Game/Dev_Content/Structs/S_SubStats_All` (`self.SubStats_Additive`))))) (`local.Amount`))))))

(fn `ModifyBaseDamageMultiplier`
  (params (Amount :type "Float (double-precision)") (`Mod Type` :type "/Game/Dev_Content/Enums/E_ModType Enum" :default "NewEnumerator0"))
  (switch `/Game/Dev_Content/Enums/E_ModType` `Mod Type`
    (:`NewEnumerator0`
      (setmembers `/Game/Dev_Content/Structs/S_SubStats_Offensive` :`StructRef` (`.Offensive_9_D88559E34BB9C3BDFF9365BCC90D44E4` (break `/Game/Dev_Content/Structs/S_SubStats_All` (`self.SubStats_Additive`))) :`BaseAttackDmgMult` (+ (`.BaseAttackDmgMult_41_F4E219434D7DCBF82BBDA4AF5C32AEDF` (break `/Game/Dev_Content/Structs/S_SubStats_Offensive` (`.Offensive_9_D88559E34BB9C3BDFF9365BCC90D44E4` (break `/Game/Dev_Content/Structs/S_SubStats_All` (`self.SubStats_Additive`))))) (`local.Amount`))))
    (:`NewEnumerator1`
      (setmembers `/Game/Dev_Content/Structs/S_SubStats_Offensive` :`StructRef` (`.Offensive_9_D88559E34BB9C3BDFF9365BCC90D44E4` (break `/Game/Dev_Content/Structs/S_SubStats_All` (`self.SubStats_Additive`))) :`BaseAttackDmgMult` (- (`.BaseAttackDmgMult_41_F4E219434D7DCBF82BBDA4AF5C32AEDF` (break `/Game/Dev_Content/Structs/S_SubStats_Offensive` (`.Offensive_9_D88559E34BB9C3BDFF9365BCC90D44E4` (break `/Game/Dev_Content/Structs/S_SubStats_All` (`self.SubStats_Additive`))))) (`local.Amount`))))))

(fn `ModifyCriticalChance`
  (params (Amount :type "Float (double-precision)") (ModType :type "/Game/Dev_Content/Enums/E_ModType Enum" :default "NewEnumerator0"))
  (switch `/Game/Dev_Content/Enums/E_ModType` ModType
    (:`NewEnumerator0`
      (setmembers `/Game/Dev_Content/Structs/S_SubStats_Offensive` :`StructRef` (`.Offensive_9_D88559E34BB9C3BDFF9365BCC90D44E4` (break `/Game/Dev_Content/Structs/S_SubStats_All` (`self.SubStats_Additive`))) :`CriticalChance` (+ (`.CriticalChance_27_13BD6E7B4853C1D64214229860612933` (break `/Game/Dev_Content/Structs/S_SubStats_Offensive` (`.Offensive_9_D88559E34BB9C3BDFF9365BCC90D44E4` (break `/Game/Dev_Content/Structs/S_SubStats_All` (`self.SubStats_Additive`))))) (`local.Amount`))))
    (:`NewEnumerator1`
      (setmembers `/Game/Dev_Content/Structs/S_SubStats_Offensive` :`StructRef` (`.Offensive_9_D88559E34BB9C3BDFF9365BCC90D44E4` (break `/Game/Dev_Content/Structs/S_SubStats_All` (`self.SubStats_Additive`))) :`CriticalChance` (- (`.CriticalChance_27_13BD6E7B4853C1D64214229860612933` (break `/Game/Dev_Content/Structs/S_SubStats_Offensive` (`.Offensive_9_D88559E34BB9C3BDFF9365BCC90D44E4` (break `/Game/Dev_Content/Structs/S_SubStats_All` (`self.SubStats_Additive`))))) (`local.Amount`))))))

(fn `ModifyDamageReduction`
  (params (Amount :type "Float (double-precision)") (`Mod Type` :type "/Game/Dev_Content/Enums/E_ModType Enum" :default "NewEnumerator0"))
  (switch `/Game/Dev_Content/Enums/E_ModType` `Mod Type`
    (:`NewEnumerator0`
      (setmembers `/Game/Dev_Content/Structs/S_SubStats_Defensive` :`StructRef` (`.Defensive_10_61502738442807B468EBCA8F9BA2D701` (break `/Game/Dev_Content/Structs/S_SubStats_All` (`self.SubStats_Additive`))) :`DamageReduction` (+ (`.DamageReduction_35_7CE2E0B24A2CDA0C5E0E719257526966` (break `/Game/Dev_Content/Structs/S_SubStats_Defensive` (`.Defensive_10_61502738442807B468EBCA8F9BA2D701` (break `/Game/Dev_Content/Structs/S_SubStats_All` (`self.SubStats_Additive`))))) (`local.Amount`))))
    (:`NewEnumerator1`
      (setmembers `/Game/Dev_Content/Structs/S_SubStats_Defensive` :`StructRef` (`.Defensive_10_61502738442807B468EBCA8F9BA2D701` (break `/Game/Dev_Content/Structs/S_SubStats_All` (`self.SubStats_Additive`))) :`DamageReduction` (- (`.DamageReduction_35_7CE2E0B24A2CDA0C5E0E719257526966` (break `/Game/Dev_Content/Structs/S_SubStats_Defensive` (`.Defensive_10_61502738442807B468EBCA8F9BA2D701` (break `/Game/Dev_Content/Structs/S_SubStats_All` (`self.SubStats_Additive`))))) (`local.Amount`))))))

(fn `ModifyElementalDamage`
  (params (Amount :type "Float (double-precision)") (ModType :type "/Game/Dev_Content/Enums/E_ModType Enum" :default "NewEnumerator0")))

(fn `ModifyHealth`
  (params (Amount :type Integer) (ModType :type "/Game/Dev_Content/Enums/E_ModType Enum" :default "NewEnumerator0"))
  (switch `/Game/Dev_Content/Enums/E_ModType` ModType
    (:`NewEnumerator0`
      (setmembers `/Game/Dev_Content/Structs/S_SubStats_Defensive` :`StructRef` (`.Defensive_10_61502738442807B468EBCA8F9BA2D701` (break `/Game/Dev_Content/Structs/S_SubStats_All` (`self.SubStats_Additive`))) :`MaxHealth` (+ (`.MaxHealth_6_A72FEEB1411FA52892BB53952A4F1E3E` (break `/Game/Dev_Content/Structs/S_SubStats_Defensive` (`.Defensive_10_61502738442807B468EBCA8F9BA2D701` (break `/Game/Dev_Content/Structs/S_SubStats_All` (`self.SubStats_Additive`))))) (`local.Amount`))))
    (:`NewEnumerator1`
      (setmembers `/Game/Dev_Content/Structs/S_SubStats_Defensive` :`StructRef` (`.Defensive_10_61502738442807B468EBCA8F9BA2D701` (break `/Game/Dev_Content/Structs/S_SubStats_All` (`self.SubStats_Additive`))) :`MaxHealth` (- (`.MaxHealth_6_A72FEEB1411FA52892BB53952A4F1E3E` (break `/Game/Dev_Content/Structs/S_SubStats_Defensive` (`.Defensive_10_61502738442807B468EBCA8F9BA2D701` (break `/Game/Dev_Content/Structs/S_SubStats_All` (`self.SubStats_Additive`))))) (`local.Amount`))))))

(fn `ModifyIntellect`
  (params (Amount :type Integer) (ModType :type "/Game/Dev_Content/Enums/E_ModType Enum" :default "NewEnumerator0"))
  (`|ExecutionSequence`
    (:`then_0`
      (switch `/Game/Dev_Content/Enums/E_ModType` (`local.ModType`)
        (:`NewEnumerator0`
          (setmembers `/Game/Dev_Content/Structs/S_PrimaryStats` :`StructRef` (`self.Primary_Additive`) :`Intellect` (+ (`.Intellect_8_DEE1C50941A32BCA0CC4FEBAB9FD97C5` (break `/Game/Dev_Content/Structs/S_PrimaryStats` (`self.Primary_Additive`))) (`local.Amount`))))
        (:`NewEnumerator1`
          (setmembers `/Game/Dev_Content/Structs/S_PrimaryStats` :`StructRef` (`self.Primary_Additive`) :`Intellect` (- (`.Intellect_8_DEE1C50941A32BCA0CC4FEBAB9FD97C5` (break `/Game/Dev_Content/Structs/S_PrimaryStats` (`self.Primary_Additive`))) (`local.Amount`))))))
    (:`then_1`
      (`self.ModifiyEnergy` (`KismetMathLibrary.Round` (* (`self.GetEnergy`) (/ (`KismetMathLibrary.Conv_IntToDouble` (* (`local.Amount`) (`.MaxEnergy_31_3BF29F7D497C1C0505D8FE857D2DA1ED` (break `/Game/Dev_Content/Structs/S_SubStats_Defensive` (`.Defensive_10_61502738442807B468EBCA8F9BA2D701` (break `/Game/Dev_Content/Structs/S_SubStats_All` (`self.Substats_Modifiers`))))))) 100.0))) (`local.ModType`)))))

(fn `ModifyPrimaryStats`
  (params (StrMod :type Integer) (AgiMod :type Integer) (IntMod :type Integer) (ModType :type "/Game/Dev_Content/Enums/E_ModType Enum" :default "NewEnumerator0"))
  (`|ExecutionSequence`
    (:`then_0`
      (`self.ModifyStrength` (`local.StrMod`) (`local.ModType`)))
    (:`then_1`
      (`self.ModifyAgility` (`local.AgiMod`) (`local.ModType`)))
    (:`then_2`
      (`self.ModifyIntellect` (`local.IntMod`) (`local.ModType`)))))

(fn `ModifySpellDamage`
  (params (Amount :type Integer) (ModType :type "/Game/Dev_Content/Enums/E_ModType Enum" :default "NewEnumerator0")))

(fn `ModifyStrength`
  (params (Amount :type Integer) (ModType :type "/Game/Dev_Content/Enums/E_ModType Enum" :default "NewEnumerator0"))
  (bind _primary_additive_strength (break `/Game/Dev_Content/Structs/S_PrimaryStats` (`self.Primary_Additive`)))
  (bind _amount (`local.Amount`))
  (bind _primary_additive_strength_2 (break `/Game/Dev_Content/Structs/S_PrimaryStats` (`self.Primary_Additive`)))
  (bind ((`BaseAttackDamage_Min_29_4E0461DD4A53AE0F8637378B561D89A4` _baseattackdamage_min) (`BaseAttackDamage_Max_30_527B76E540F80C7F4FC7E4898C7C70F0` _baseattackdamage_max)) (break `/Game/Dev_Content/Structs/S_SubStats_Offensive` (`.Offensive_9_D88559E34BB9C3BDFF9365BCC90D44E4` (break `/Game/Dev_Content/Structs/S_SubStats_All` (`self.Substats_Modifiers`)))))
  (`|ExecutionSequence`
    (:`then_0`
      (switch `/Game/Dev_Content/Enums/E_ModType` (`local.ModType`)
        (:`NewEnumerator0`
          (setmembers `/Game/Dev_Content/Structs/S_PrimaryStats` :`StructRef` (`self.Primary_Additive`) :`Strength` (+ _primary_additive_strength_2 (`local.Amount`))))
        (:`NewEnumerator1`
          (setmembers `/Game/Dev_Content/Structs/S_PrimaryStats` :`StructRef` (`self.Primary_Additive`) :`Strength` (- _primary_additive_strength (`local.Amount`))))))
    (:`then_1`
      (`self.ModifyAttackDamage` (* _amount _baseattackdamage_min) (* _amount _baseattackdamage_max) (`local.ModType`)))
    (:`then_2`
      (`self.ModifyHealth` (* (`local.Amount`) (`.MaxHealth_6_A72FEEB1411FA52892BB53952A4F1E3E` (break `/Game/Dev_Content/Structs/S_SubStats_Defensive` (`.Defensive_10_61502738442807B468EBCA8F9BA2D701` (break `/Game/Dev_Content/Structs/S_SubStats_All` (`self.Substats_Modifiers`)))))) (`local.ModType`)))))