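; Actor component that manages its owning character's standing and crouched walk speeds through two multipliers.
; On BeginPlay it caches the CharacterMovementComponent and both default max speeds.
; Set and Modify functions change the main or additive multiplier, then reapply each default times both multipliers.
; ModifyMainMultiplier computes its result from the additive multiplier rather than the current main value.
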(event `self.ReceiveBeginPlay`
  (bind _output_get (set `self.Ref_CharacterMovementComponent` (`Actor.GetComponentByClass` (`self.GetOwner`) "/Script/Engine.CharacterMovementComponent")))
  (set `self.WalkSpeed_S_Default` (`CharacterMovementComponent.MaxWalkSpeed` _output_get))
  (set `self.WalkSpeed_C_Default` (`CharacterMovementComponent.MaxWalkSpeedCrouched` _output_get)))

(fn `ModifyAdditiveMultiplier`
  (params (Value :type "Float (double-precision)") (ModType :type "/Game/Dev_Content/Enums/E_ModType Enum" :default "NewEnumerator0"))
  (bind _value (`local.Value`))
  (set `self.Multiplier_Additive` (select `/Game/Dev_Content/Enums/E_ModType` (`local.ModType`) :`NewEnumerator0` (+ (`self.Multiplier_Additive`) _value) :`NewEnumerator1` (- (`self.Multiplier_Additive`) _value)))
  (`self.SetOwnerWalkSpeed`))

(fn `ModifyMainMultiplier`
  (params (Value :type "Float (double-precision)") (ModType :type "/Game/Dev_Content/Enums/E_ModType Enum" :default "NewEnumerator0"))
  (bind _value (`local.Value`))
  (set `self.Multiplier_Main` (select `/Game/Dev_Content/Enums/E_ModType` (`local.ModType`) :`NewEnumerator0` (+ (`self.Multiplier_Additive`) _value) :`NewEnumerator1` (- (`self.Multiplier_Additive`) _value)))
  (`self.SetOwnerWalkSpeed`))

(fn `SetAdditiveMultiplier`
  (params (Value :type "Float (double-precision)"))
  (set `self.Multiplier_Additive` Value)
  (`self.SetOwnerWalkSpeed`))

(fn `SetMainMultiplier`
  (params (Value :type "Float (double-precision)"))
  (set `self.Multiplier_Main` Value)
  (`self.SetOwnerWalkSpeed`))

(fn `SetOwnerWalkSpeed`
  (`/Engine/EditorBlueprintResources/StandardMacros.IsValid` (`self.Ref_CharacterMovementComponent`)
    (:`Is Valid`
      (set `CharacterMovementComponent.MaxWalkSpeed` (* (`self.WalkSpeed_S_Default`) (`self.Multiplier_Main`) (`self.Multiplier_Additive`)) (`self.Ref_CharacterMovementComponent`))
      (set `CharacterMovementComponent.MaxWalkSpeedCrouched` (* (`self.WalkSpeed_C_Default`) (`self.Multiplier_Main`) (`self.Multiplier_Additive`)) (`self.Ref_CharacterMovementComponent`)))))