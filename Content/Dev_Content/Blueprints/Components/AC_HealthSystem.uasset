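; AC_HealthSystem is an actor component that tracks current and maximum health for its owner.
; On BeginPlay it sets current health from the starting value, and all changes pass through one setter that clamps between zero and max.
; Helpers add or subtract health, change the maximum with an optional refill, and report death, a safely divided percentage and both values.
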(event `self.ReceiveBeginPlay`
  (`self.SetCurrentHealthClamped` (`self.StartingHealth`)))

(fn `AddHealth`
  (params (Amount :type "Float (double-precision)"))
  (`self.SetCurrentHealthClamped` (+ Amount (`self.CurrentHealth`))))

(fn `GetHealthPercentage`
  (returns (`Out %` :type "Float (double-precision)"))
  (return (`KismetMathLibrary.SafeDivide` (`self.CurrentHealth`) (`self.MaxHealth`))))

(fn `GetHealthStats`
  (returns (MaxHealth :type "Float (double-precision)") (CurrentHealth :type "Float (double-precision)"))
  (return (`self.MaxHealth`) (`self.CurrentHealth`)))

(fn `IsDead?`
  (returns (Out :type Boolean))
  (return (<= (`self.CurrentHealth`) 0.0)))

(fn `SetCurrentHealthClamped`
  (params (NewAmount :type "Float (double-precision)"))
  (set `self.CurrentHealth` (`KismetMathLibrary.FClamp` NewAmount 0.0 (`self.MaxHealth`))))

(fn `SetMaxHealth`
  (params (NewMax :type "Float (double-precision)") (`SetCurrentToMax?` :type Boolean :default true))
  (bind _output_get (set `self.MaxHealth` NewMax))
  (if `SetCurrentToMax?`
    (`self.SetCurrentHealthClamped` _output_get)))

(fn `SubtractHealth`
  (params (Amount :type "Float (double-precision)"))
  (`self.SetCurrentHealthClamped` (- (`self.CurrentHealth`) Amount)))