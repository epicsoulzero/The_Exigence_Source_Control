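; Skill component that drops a stun trap at the user's position.
; UseSkill checks CanUseSkill, spawns a BP_BaseTrap slightly above the user with its collision profile, stun duration and lifespan, then resets the cooldown.
; The hit and start points do not affect placement.
; GetVelocity computes a horizontal velocity to cover the distance to a hit point in a given time, but is unused.
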(fn `GetVelocity`
  (params (HitPoint :type "Vector Structure") (StartPoint :type "Vector Structure") (TravelTime :type "Float (double-precision)" :default 0.5))
  (returns (Out :type "Vector Structure"))
  (locals (Height :type "Float (double-precision)") (Distance :type "Float (double-precision)"))
  (bind (_startpoint_x _startpoint_y _startpoint_z) (`KismetMathLibrary.BreakVector` (`local.StartPoint`)))
  (bind (_hitpoint_x _hitpoint_y _hitpoint_z) (`KismetMathLibrary.BreakVector` (`local.HitPoint`)))
  (bind (_startpoint_x_2 _startpoint_y_2) (`KismetMathLibrary.BreakVector` (`local.StartPoint`)))
  (bind (_hitpoint_x_2 _hitpoint_y_2 _hitpoint_z_2) (`KismetMathLibrary.BreakVector` (`local.HitPoint`)))
  (bind (_startpoint_x_3 _startpoint_y_3) (`KismetMathLibrary.BreakVector` (`local.StartPoint`)))
  (`|ExecutionSequence`
    (:`then_0`
      (set `local.Height` _startpoint_z)
      (set `local.Distance` (`KismetMathLibrary.Vector_Distance` (`KismetMathLibrary.MakeVector` _startpoint_x_3 _startpoint_y_3 _hitpoint_z_2) (`KismetMathLibrary.MakeVector` _hitpoint_x_2 _hitpoint_y_2 _hitpoint_z_2))))
    (:`then_1`
      (return (* (`KismetMathLibrary.GetDirectionUnitVector` (`KismetMathLibrary.MakeVector` _startpoint_x_2 _startpoint_y_2 _hitpoint_z) (`KismetMathLibrary.MakeVector` _hitpoint_x _hitpoint_y _hitpoint_z)) (/ (`local.Distance`) (* (`local.TravelTime`) (`KismetMathLibrary.DegCos` 0.0))))))))

(fn `UseSkill`
  (params (User :type "Actor Object Reference") (HitPoint :type "Vector Structure") (StartPoint :type "Vector Structure"))
  (bind _out (`self.CanUseSkill?` User))
  (if _out
    (`|SpawnActorFromClass` "/Game/Dev_Content/Blueprints/Miscellaneous/BP_BaseTrap.BP_BaseTrap_C" (`KismetMathLibrary.MakeTransform` (+ (`Actor.K2_GetActorLocation` User) (* (`KismetMathLibrary.Vector_Up`) 50.0))) "AlwaysSpawn" "OverrideRootScale" null (`self.Collision Profile Name`) (`self.StunDuration`) (`self.Duration`) (0.0 0.0 0.0) null)
    (`self.ResetCD` 1.0)))