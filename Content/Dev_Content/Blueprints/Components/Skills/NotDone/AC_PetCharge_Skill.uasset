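; AC_PetCharge_Skill is a skill component that orders the user's hunter pet to charge a target or location.
; UseSkill checks CanUseSkill, finds the pet through the user's AC_PetSystem, and passes the hit data to EventInitChargeSkill.
; It then adds a long-duration movement modifier to the pet and resets the cooldown.
; These later steps run even if the pet lookup fails, which only prints debug messages.
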(fn `UseSkill`
  (params (User :type "Actor Object Reference") (HitTarget :type "Actor Object Reference") (HitLocation :type "Vector Structure"))
  (bind _returnvalue (`Actor.GetComponentByClass` (`local.User`) "/Game/Dev_Content/Blueprints/Components/Skills/AC_PetSystem.AC_PetSystem_C"))
  (bind _out (`self.CanUseSkill?` User))
  (if _out
    (`|ExecutionSequence`
      (:`then_0`
        (`/Engine/EditorBlueprintResources/StandardMacros.IsValid` _returnvalue
          (:`Is Valid`
            (bind _asbp_hunter_pet (cast `/Game/Dev_Content/Blueprints/Pet/HunterPet/BP_HunterPet` (`/Game/Dev_Content/Blueprints/Components/Skills/AC_PetSystem.Ref_Pet` _returnvalue))
              (:`then`
                (bind _output_get (set `self.Ref_Pet` _asbp_hunter_pet))
                (`/Game/Dev_Content/Blueprints/Pet/HunterPet/BP_HunterPet.Event_InitChargeSkill` _output_get (`local.HitTarget`) (`local.HitLocation`)))
              (:`CastFailed`
                (`KismetSystemLibrary.PrintString` "Cast failed" (`self.ShowDebugs?`)))))
          (:`Is Not Valid`
            (`KismetSystemLibrary.PrintString` "Component not valid" (`self.ShowDebugs?`)))))
      (:`then_1`
        (`|AddComponentByClass` (`self.Ref_Pet`) "/Game/Dev_Content/Blueprints/Components/StatusEffects/AC_MovementModifier_SE.AC_MovementModifier_SE_C" 1.0 0.5 null 0.0 99.0))
      (:`then_2`
        (`self.ResetCD` 1.0)))
    (else
      (`KismetSystemLibrary.PrintString` "Unable to use skill" (`self.ShowDebugs?`) false (struct :`G` 0.5 :`B` 1.0 :`A` 1.0)))))