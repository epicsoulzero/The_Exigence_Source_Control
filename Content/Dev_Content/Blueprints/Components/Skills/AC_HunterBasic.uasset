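; Hunter basic skill component that fires a projectile with an on-hit effect in a given direction.
; UseSkill checks CanUseSkill, applies a movement modifier status effect to the user for the cast time, triggers the shot event and resets the cooldown.
; Despite its name, the DelayedShot event spawns the projectile without a delay, passing it the owner, damage range, direction, collision profile and a fixed speed.
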(event `Event_DelayedShot`
  (params (Owner :type "Actor Object Reference") (StartPoint :type "Vector Structure") (Direction :type "Vector Structure"))
  (bind (_x _y) (`KismetMathLibrary.BreakVector2D` (`self.Damage`)))
  (`|SpawnActorFromClass` "/Game/Dev_Content/Blueprints/Miscellaneous/BP_Projectile_WithOnHitEffect.BP_Projectile_WithOnHitEffect_C" (`KismetMathLibrary.MakeTransform` StartPoint) "AlwaysSpawn" "OverrideRootScale" Owner (`KismetMathLibrary.MakeVector2D` _x _y) 2000.0 Direction (`self.Collision Profile Name`) null))

(fn `UseSkill`
  (params (User :type "Actor Object Reference") (Direction :type "Vector Structure") (StartPoint :type "Vector Structure"))
  (bind _out (`self.CanUseSkill?` User))
  (if _out
    (`|ExecutionSequence`
      (:`then_0`
        (`|AddComponentByClass` (`local.User`) "/Game/Dev_Content/Blueprints/Components/StatusEffects/AC_MovementModifier_SE.AC_MovementModifier_SE_C" 0.0 0.0 null 0.0 (`self.CastTime`)))
      (:`then_1`
        (`self.Event_DelayedShot` (`local.User`) (`local.StartPoint`) (`local.Direction`)))
      (:`then_2`
        (`self.ResetCD` 1.0)))))