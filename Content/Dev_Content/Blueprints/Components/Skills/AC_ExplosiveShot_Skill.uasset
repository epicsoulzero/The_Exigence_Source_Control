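; Skill component for an explosive shot that fires an area-of-effect projectile after a cast time.
; UseSkill checks CanUseSkill, then applies a movement modifier status effect to the user for the cast duration, starts the delayed shot and immediately resets the cooldown.
; After the delay, the event spawns BP_Projectile_AOE offset along the aim direction, passing in the skill's damage, radius, speed and collision settings.
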(event `Event_DelayedShot`
  (params (Direction :type "Vector Structure") (StartSpawn :type "Vector Structure"))
  (`KismetSystemLibrary.Delay` (`self.CastTime`))
  (`|SpawnActorFromClass` "/Game/Dev_Content/Blueprints/Miscellaneous/BP_Projectile_AOE.BP_Projectile_AOE_C" (`KismetMathLibrary.MakeTransform` (+ (* Direction (`self.Offset`)) StartSpawn)) "AlwaysSpawn" "OverrideRootScale" null (`self.Duration`) (`self.Range`) (`self.AoeDamage`) (`self.Hittable Objects`) (`self.InitialDamage`) (`self.Speed`) Direction (`self.CollisionProfileName`) null))

(fn `UseSkill`
  (params (User :type "Actor Object Reference") (Direction :type "Vector Structure") (StartSpawn :type "Vector Structure"))
  (bind _out (`self.CanUseSkill?` User))
  (if _out
    (`|ExecutionSequence`
      (:`then_0`
        (`|AddComponentByClass` (`local.User`) "/Game/Dev_Content/Blueprints/Components/StatusEffects/AC_MovementModifier_SE.AC_MovementModifier_SE_C" 0.0 0.0 null 0.0 (`self.CastTime`))
        (`self.Event_DelayedShot` (`local.Direction`) (`local.StartSpawn`)))
      (:`then_1`
        (`self.ResetCD` 1.0)))
    (else
      (`KismetSystemLibrary.PrintString` "Unable to use skill" (`self.ShowDebugs?`) false (struct :`G` 0.5 :`B` 1.0 :`A` 1.0)))))