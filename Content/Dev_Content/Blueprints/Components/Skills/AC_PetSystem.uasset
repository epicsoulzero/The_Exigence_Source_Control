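; Skill component that spawns and tracks a single pet for its owning character, optionally at BeginPlay.
; If no valid pet exists, a retriggerable delay precedes a downward line trace against WorldStatic from randomized points around the owner.
; The pet spawns just above the hit location and receives the owning BP_BaseCharacter as its owner.
; KillPet destroys it through massive damage credited to a given dealer.
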(event `self.ReceiveBeginPlay`
  (if (`self.SpawnOnStart?`)
    (`self.Event_SpawnPet`)))

(event `Event_SpawnPet`
  (bind _returnvalue (`KismetMathLibrary.Vector_Up`))
  (bind _returnvalue_2 (+ (* (`KismetMathLibrary.RandomUnitVector`) 200.0) (`Actor.K2_GetActorLocation` (`self.GetOwner`))))
  (`/Engine/EditorBlueprintResources/StandardMacros.IsValid` (`self.Ref_Pet`)
    (:`Is Not Valid`
      (`KismetSystemLibrary.RetriggerableDelay` (`self.SpawnDelay`))
      (bind _outhit (`KismetSystemLibrary.LineTraceSingleForObjects` :`Start` (+ _returnvalue_2 (* _returnvalue 200.0)) :`End` (- _returnvalue_2 (* _returnvalue 10900.0)) :`ObjectTypes` (`|MakeArray` "ObjectTypeQuery1" :!type "EObjectTypeQuery Enum") :`DrawTime` 10.0))
      (bind _returnvalue_3 (`|SpawnActorFromClass` (`self.PetClass`) (`KismetMathLibrary.MakeTransform` (+ (`.Location` (`GameplayStatics.BreakHitResult` _outhit)) (* (`KismetMathLibrary.Vector_Up`) 50.0))) "AlwaysSpawn" "OverrideRootScale" null self null))
      (bind _output_get (set `self.Ref_Pet` _returnvalue_3))
      (bind _asbp_base_character (cast `/Game/Dev_Content/Blueprints/Chars/BP_BaseCharacter` (`self.GetOwner`)))
      (set `/Game/Dev_Content/Blueprints/Pet/BP_BasePet.MyOwner` _asbp_base_character _output_get))))

(fn `KillPet`
  (params (Dealer :type "Actor Object Reference"))
  (`/Engine/EditorBlueprintResources/StandardMacros.IsValid` (`self.Ref_Pet`)
    (:`Is Valid`
      (message `/Game/Dev_Content/Blueprints/Interfaces/BPI_Damageable.TakeDamage` (`self.Ref_Pet`) 9999999.0 Dealer))))