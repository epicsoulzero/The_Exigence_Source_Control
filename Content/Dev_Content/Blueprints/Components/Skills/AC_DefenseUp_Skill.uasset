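; AC_DefenseUp_Skill is a skill component that grants its user a temporary defense-up status effect.
; UseSkill checks CanUseSkill, then adds an AC_DefenseUp_SE component to the user with the skill's multiplier and duration.
; It registers that effect with the user's AC_StatusEffect_Manager and resets the cooldown, or prints a debug message when the skill cannot be used.
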(fn `UseSkill`
  (params (User :type "Actor Object Reference"))
  (bind _user (`local.User`))
  (bind _out (`self.CanUseSkill?` User))
  (if _out
    (bind _returnvalue (`|AddComponentByClass` _user "/Game/Dev_Content/Blueprints/Components/StatusEffects/AC_DefenseUp_SE.AC_DefenseUp_SE_C" (`self.Multiplier`) null 0.0 (`self.Duration`)))
    (`/Game/Dev_Content/Blueprints/Components/StatusEffects/AC_StatusEffect_Manager.AddEffect` (`Actor.GetComponentByClass` _user "/Game/Dev_Content/Blueprints/Components/StatusEffects/AC_StatusEffect_Manager.AC_StatusEffect_Manager_C") _returnvalue)
    (`self.ResetCD` 1.0)
    (else
      (`KismetSystemLibrary.PrintString` (`KismetStringLibrary.Concat_StrStr` "Unable to use: " (`self.GetDisplayName`)) (`self.ShowDebugs?`) false (struct :`G` 0.5 :`B` 1.0 :`A` 1.0)))))