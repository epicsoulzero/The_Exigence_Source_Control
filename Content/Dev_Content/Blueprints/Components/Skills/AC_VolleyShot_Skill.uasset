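; Skill component for an area volley shot that rains arrows on a target point, dealing repeated damage over a duration.
; UseSkill stores the point, applies a movement-modifier status effect to the user for the cast time, starts the tick event and resets cooldown.
; After the cast delay, each tick spawns cosmetic dummy arrows overhead and applies random damage through a capsule overlap.
; Ticks loop by retriggerable delay, splitting the duration evenly across the tick count.
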(event `Event_StartVolleyTick`
  (bind (_damage_x _damage_y) (`KismetMathLibrary.BreakVector2D` (`self.Damage`)))
  (`KismetSystemLibrary.Delay` (`self.CastTime`))
  (`self.SpawnDummyArrows` :!label _label)
  (if (`self.ShowDebugs?`)
    (`KismetSystemLibrary.DrawDebugCircle` (`self.Hit Point`) (`self.Range`) 50 (struct :`R` 1.0 :`G` 1.0 :`A` 1.0) (* (`self.GetTimePerTick`) 0.8) 3.0 (1.0 0.0 0.0) (0.0 1.0 0.0) true))
  (bind _outactors (`KismetSystemLibrary.CapsuleOverlapActors` (`self.Hit Point`) (`self.Range`) (`self.CheckHeight`) (`self.HittableObjects`)))
  (for _array_element _outactors
    (message `/Game/Dev_Content/Blueprints/Interfaces/BPI_Damageable.TakeDamage` _array_element (`KismetMathLibrary.Conv_IntToDouble` (`KismetMathLibrary.Round` (`KismetMathLibrary.RandomFloatInRange` _damage_x _damage_y))) (`self.GetOwner`)))
  (bind _result (`/Engine/EditorBlueprintResources/StandardMacros.IncrementInt` (`self.CurrentTickCount`))
    (:`  `
      (if (< _result (`self.TickCount`))
        (`KismetSystemLibrary.RetriggerableDelay` (`self.GetTimePerTick`))
        (goto _label)))))

(fn `GetTimePerTick`
  (returns (Out :type "Float (double-precision)"))
  (return (/ (`self.Duration`) (`self.TickCount`))))

(fn `SpawnDummyArrows`
  (bind _checkheight (`self.CheckHeight`))
  (for _ (range (+ (`KismetMathLibrary.RandomIntegerInRange` 10 20) 1))
    (`|SpawnActorFromClass` "/Game/BP_DummyArrow.BP_DummyArrow_C" (`KismetMathLibrary.MakeTransform` (+ (+ (* (`KismetMathLibrary.RandomFloatInRange` (- _checkheight 10.0) (+ _checkheight 10.0)) (`KismetMathLibrary.Vector_Up`)) (`self.Hit Point`)) (* (`KismetMathLibrary.RandomFloatInRange` 0.0 (* (`self.Range`) 0.9)) (`KismetMathLibrary.Vector_Normal2D` (`KismetMathLibrary.RandomUnitVector`))))) "AlwaysSpawn" "OverrideRootScale" null null)))

(fn `UseSkill`
  (params (User :type "Actor Object Reference") (HitPoint :type "Vector Structure"))
  (bind _out (`self.CanUseSkill?` User))
  (if _out
    (`|ExecutionSequence`
      (:`then_0`
        (set `self.Hit Point` (`local.HitPoint`))
        (set `self.CurrentTickCount` 0))
      (:`then_1`
        (`|AddComponentByClass` (`local.User`) "/Game/Dev_Content/Blueprints/Components/StatusEffects/AC_MovementModifier_SE.AC_MovementModifier_SE_C" 0.0 0.0 null 0.0 (`self.CastTime`)))
      (:`then_2`
        (`self.Event_StartVolleyTick`))
      (:`then_3`
        (`self.ResetCD` 1.0)))
    (else
      (`KismetSystemLibrary.PrintString` "Unable to use skill" (`self.ShowDebugs?`) false (struct :`G` 0.5 :`B` 1.0 :`A` 1.0)))))