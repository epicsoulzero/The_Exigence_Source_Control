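; Multi-shot skill component that fires a fan of projectiles around the aim direction.
; UseSkill, gated by CanUseSkill, puts a movement modifier status effect on the user for the cast time, starts the delayed volley and resets the cooldown immediately.
; After the cast delay, SpawnArrows spreads BP_Projectile actors evenly across Angle, centred by yaw rotation, each offset from the start point and given the skill's damage, speed and collision profile.
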(event `self.ReceiveTick`
  (params (DeltaSeconds :type "Float (single-precision)"))
  (`parent.ReceiveTick` DeltaSeconds))

(event `DelayedSpawnArrows`
  (params (Direction :type "Vector Structure") (StartSpawn :type "Vector Structure"))
  (`KismetSystemLibrary.Delay` (`self.CastTime`))
  (`self.SpawnArrows` Direction StartSpawn))

(fn `SpawnArrows`
  (params (Direction :type "Vector Structure") (StartSpawn :type "Vector Structure"))
  (bind _returnvalue (- (`self.ArrowCount`) 1))
  (bind _returnvalue_2 (/ (`self.Angle`) _returnvalue))
  (for _index (range (`self.ArrowCount`))
    (bind _returnvalue_3 (`KismetMathLibrary.GreaterGreater_VectorRotator` (`local.Direction`) (`KismetMathLibrary.MakeRotator` 0.0 0.0 (- (* _index _returnvalue_2) (* (/ (`KismetMathLibrary.Conv_IntToDouble` _returnvalue) 2.0) _returnvalue_2)))))
    (`|SpawnActorFromClass` "/Game/Dev_Content/Blueprints/Miscellaneous/BP_Projectile.BP_Projectile_C" (`KismetMathLibrary.MakeTransform` (+ (* _returnvalue_3 (`self.Offset`)) (`local.StartSpawn`))) "AlwaysSpawn" "OverrideRootScale" null (`self.Damage`) (`self.Speed`) _returnvalue_3 (`self.CollisionProfileName`) null)))

(fn `UseSkill`
  (params (User :type "Actor Object Reference") (Direction :type "Vector Structure") (StartSpawn :type "Vector Structure"))
  (bind _out (`self.CanUseSkill?` User))
  (if _out
    (`|ExecutionSequence`
      (:`then_0`
        (`|AddComponentByClass` (`local.User`) "/Game/Dev_Content/Blueprints/Components/StatusEffects/AC_MovementModifier_SE.AC_MovementModifier_SE_C" 0.0 0.0 null 0.0 (`self.CastTime`)))
      (:`then_1`
        (`self.DelayedSpawnArrows` (`local.Direction`) (`local.StartSpawn`)))
      (:`then_2`
        (`self.ResetCD` 1.0)))
    (else
      (`KismetSystemLibrary.PrintString` "Unable to use skill" (`self.ShowDebugs?`) false (struct :`G` 0.5 :`B` 1.0 :`A` 1.0)))))