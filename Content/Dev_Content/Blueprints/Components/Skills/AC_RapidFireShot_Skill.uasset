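; Skill component that fires a rapid burst of BP_Projectile shots over the skill's cast time.
; UseSkill checks CanUseSkill, applies a movement modifier to the user for the cast, starts the burst and resets the cooldown.
; A retriggerable-delay loop spaces the shots evenly, reusing the start point and direction passed in.
; Helper functions derive a flattened cursor aim, falling back to LastDirection, and an offset start point.
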(event `Event_DelayedShot`
  (params (StartPoint :type "Vector Structure") (Direction :type "Vector Structure"))
  (`|SpawnActorFromClass` "/Game/Dev_Content/Blueprints/Miscellaneous/BP_Projectile.BP_Projectile_C" (`KismetMathLibrary.MakeTransform` (+ StartPoint (* Direction (`self.Offset`)))) "AlwaysSpawn" "OverrideRootScale" null (`self.Damage Min Max`) 2000.0 Direction (`self.Collision Profile Name`) null :!label _label)
  (`/Engine/EditorBlueprintResources/StandardMacros.DecrementInt` (`self.RemainingShots`)
    (:`  `
      (if (> (`self.RemainingShots`) 0)
        (`KismetSystemLibrary.RetriggerableDelay` (`self.GetIntervals`))
        (goto _label)))))

(fn `GetIntervals`
  (returns (Out :type "Float (double-precision)"))
  (return (`KismetMathLibrary.SafeDivide` (`self.CastTime`) (`KismetMathLibrary.Conv_IntToDouble` (- (`self.ShotCount`) 1)))))

(fn `GetShootDirection`
  (params (Controller :type "PlayerController Object Reference"))
  (returns (Out :type "Vector Structure"))
  (locals (CursorHitLoc :type "Vector Structure"))
  (bind (_hitresult _returnvalue) (`PlayerController.GetHitResultUnderCursorByChannel` Controller "TraceTypeQuery1" true))
  (bind (_returnvalue_x _returnvalue_y) (`KismetMathLibrary.BreakVector` (`Actor.K2_GetActorLocation` (`Controller.K2_GetPawn` Controller))))
  (set `local.CursorHitLoc` (`.Location` (`GameplayStatics.BreakHitResult` _hitresult)))
  (return (select `bool` _returnvalue :`false` (`self.LastDirection`) :`true` (`KismetMathLibrary.GetDirectionUnitVector` (`KismetMathLibrary.MakeVector` _returnvalue_x _returnvalue_y (.z (`local.CursorHitLoc`))) (`local.CursorHitLoc`)))))

(fn `GetStartPoint`
  (params (Offsets :type "Vector Structure") (ActorLoc :type "Vector Structure"))
  (returns (Out :type "Vector Structure"))
  (bind (_offsets_x _offsets_y _offsets_z) (`KismetMathLibrary.BreakVector` (`local.Offsets`)))
  (return (+ ActorLoc (* (`self.LastDirection`) _offsets_x) (* (`KismetMathLibrary.Vector_Up`) _offsets_z))))

(fn `UseSkill`
  (params (User :type "Actor Object Reference") (StartPoint :type "Vector Structure") (Direction :type "Vector Structure"))
  (returns (Return :type Boolean))
  (bind _out (`self.CanUseSkill?` User))
  (if _out
    (`|ExecutionSequence`
      (:`then_0`
        (set `self.RemainingShots` (`self.ShotCount`)))
      (:`then_1`
        (`|AddComponentByClass` (`local.User`) "/Game/Dev_Content/Blueprints/Components/StatusEffects/AC_MovementModifier_SE.AC_MovementModifier_SE_C" 0.0 0.0 null 0.0 (`self.CastTime`)))
      (:`then_2`
        (`self.Event_DelayedShot` (`local.StartPoint`) (`local.Direction`)))
      (:`then_3`
        (`self.ResetCD` 1.0))
      (:`then_4`
        (return true)))
    (else
      (`KismetSystemLibrary.PrintString` "Unable to use skill" (`self.ShowDebugs?`) false (struct :`G` 0.5 :`B` 1.0 :`A` 1.0))
      (return false))))