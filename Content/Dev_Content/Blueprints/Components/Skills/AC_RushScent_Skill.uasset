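; Skill component for Rush Scent, which applies a timed movement modifier to the user and their pet.
; UseSkill checks CanUseSkill, then adds an AC_MovementModifier_SE component to the user with an additive multiplier and duration.
; It adds the same effect to the pet referenced by the user's AC_PetSystem, if both are valid, then resets the cooldown.
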(fn `UseSkill`
  (params (User :type "Actor Object Reference"))
  (bind _returnvalue (`Actor.GetComponentByClass` (`local.User`) "/Game/Dev_Content/Blueprints/Components/Skills/AC_PetSystem.AC_PetSystem_C"))
  (bind _ref_pet (`/Game/Dev_Content/Blueprints/Components/Skills/AC_PetSystem.Ref_Pet` _returnvalue))
  (bind _out (`self.CanUseSkill?` User))
  (if _out
    (`|ExecutionSequence`
      (:`then_0`
        (`|AddComponentByClass` (`local.User`) "/Game/Dev_Content/Blueprints/Components/StatusEffects/AC_MovementModifier_SE.AC_MovementModifier_SE_C" 1.0 (`self.Multiplier_Additive`) null 0.0 (`self.Duration`)))
      (:`then_1`
        (`/Engine/EditorBlueprintResources/StandardMacros.IsValid` _returnvalue
          (:`Is Valid`
            (`/Engine/EditorBlueprintResources/StandardMacros.IsValid` _ref_pet
              (:`Is Valid`
                (`|AddComponentByClass` _ref_pet "/Game/Dev_Content/Blueprints/Components/StatusEffects/AC_MovementModifier_SE.AC_MovementModifier_SE_C" 1.0 (`self.Multiplier_Additive`) null 0.0 (`self.Duration`)))))))
      (:`then_2`
        (`self.ResetCD` 1.0)))))