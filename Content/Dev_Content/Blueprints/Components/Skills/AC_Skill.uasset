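; Skill component that gates ability use behind a cooldown and a mana cost.
; Tick counts the cooldown down, ResetCD starts it at a multiple of the base Cooldown, and GetPercentCD returns the clamped fraction remaining.
; CanUseSkill validates the user and cooldown, then deducts mana through the user's AC_ManaSystem, so a successful check spends mana but leaves the cooldown untouched.
; Debug prints report cooldowns and failed uses.
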(event `self.ReceiveTick`
  (params (DeltaSeconds :type "Float (single-precision)"))
  (set `self.DeltaTime` DeltaSeconds)
  (`|ExecutionSequence`
    (:`then_0`
      (if (`self.IsOnCD?`)
        (bind _output_get (set `self.CooldownTimer` (- (`self.CooldownTimer`) (`self.DeltaTime`))))
        (`KismetSystemLibrary.PrintString` (`KismetStringLibrary.Concat_StrStr` (`self.GetDisplayName`) (`KismetStringLibrary.Conv_DoubleToString` _output_get)) (`self.ShowDebugs?`) true (struct :`G` 0.5 :`B` 1.0 :`A` 1.0) 0.0)))))

(fn `CanUseSkill?`
  (params (User :type "Actor Object Reference"))
  (returns (Out :type Boolean))
  (`/Engine/EditorBlueprintResources/StandardMacros.IsValid` User
    (:`Is Valid`
      (if (not (`self.IsOnCD?`))
        (bind _success_ (`self.CheckAndDeductCost` User))
        (if _success_
          (return true)
          (else
            (`KismetSystemLibrary.PrintString` (`KismetStringLibrary.Concat_StrStr` "Not enough mana for: " (`self.GetDisplayName`)) (`self.ShowDebugs?`) false (struct :`G` 0.5 :`B` 1.0 :`A` 1.0))
            (return false)))
        (else
          (`KismetSystemLibrary.PrintString` (`KismetStringLibrary.Concat_StrStr` (`self.GetDisplayName`) " is on cooldown") (`self.ShowDebugs?`) false (struct :`G` 0.5 :`B` 1.0 :`A` 1.0))
          (return false))))
    (:`Is Not Valid`
      (`KismetSystemLibrary.PrintString` (`KismetStringLibrary.Concat_StrStr` "User is not valid when " (`self.GetDisplayName`) " is used") true false (struct :`G` 0.5 :`B` 1.0 :`A` 1.0))
      (return false))))

(fn `CheckAndDeductCost`
  (params (User :type "Actor Object Reference"))
  (returns (`Success?` :type Boolean))
  (bind _returnvalue (`Actor.GetComponentByClass` User "/Game/Dev_Content/Blueprints/Components/AC_ManaSystem.AC_ManaSystem_C"))
  (`/Engine/EditorBlueprintResources/StandardMacros.IsValid` _returnvalue
    (:`Is Valid`
      (if (`/Game/Dev_Content/Blueprints/Components/AC_ManaSystem.HasEnoughMana?` _returnvalue (`self.Cost`))
        (`/Game/Dev_Content/Blueprints/Components/AC_ManaSystem.SubtractMana` _returnvalue (`self.Cost`))
        (return true)
        (else
          _)))
    (:`Is Not Valid`
      _))
  (return false))

(fn `GetDisplayName`
  (returns (Out :type String))
  (return (`.RightS` (`KismetStringLibrary.Split` (`KismetSystemLibrary.GetDisplayName` self) "." "IgnoreCase" "FromEnd"))))

(fn `GetPercentCD`
  (returns (Out :type "Float (double-precision)"))
  (return (`KismetMathLibrary.FClamp` (/ (`self.CooldownTimer`) (`self.Cooldown`)))))

(fn `IsOnCD?`
  (returns (Out :type Boolean))
  (return (> (`self.CooldownTimer`) 0.0)))

(fn `ResetCD`
  (params (Multiplier :type "Float (double-precision)" :default 1.0))
  (set `self.CooldownTimer` (* Multiplier (`self.Cooldown`))))