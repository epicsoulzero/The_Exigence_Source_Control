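; Projectile Blueprint that grants its owner mana when it hits an enemy.
; It overrides the parent On Hit, checks for an exact BP_EnemyCharacter class match (subclasses do not count), and adds FocusGain through the owner's AC_ManaSystem component if present.
; The parent On Hit logic then runs for every hit, whatever the target.
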(fn `On Hit`
  (params (HitActor :type "Object Object Reference"))
  (returns (`HitSuccess?` :type Boolean))
  (bind _returnvalue (`self.GetComponentByClass` (`self.GetOwner`) "/Game/Dev_Content/Blueprints/Components/AC_ManaSystem.AC_ManaSystem_C"))
  (`|ExecutionSequence`
    (:`then_0`
      (if (== (`GameplayStatics.GetObjectClass` (`local.HitActor`)) "/Game/Dev_Content/Blueprints/Chars/Enemy/BP_EnemyCharacter.BP_EnemyCharacter_C")
        (`/Engine/EditorBlueprintResources/StandardMacros.IsValid` _returnvalue
          (:`Is Valid`
            (`/Game/Dev_Content/Blueprints/Components/AC_ManaSystem.AddMana` _returnvalue (`self.FocusGain`))))))
    (:`then_1`
      (bind _hitsuccess_ (`parent.On Hit` (`local.HitActor`)))
      (return _hitsuccess_))))

(fn `UserConstructionScript`
  (`parent.UserConstructionScript`))