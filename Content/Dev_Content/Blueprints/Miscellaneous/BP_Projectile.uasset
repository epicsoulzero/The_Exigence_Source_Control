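; Projectile actor that flies along a set direction and damages whatever its box collides with.
; BeginPlay applies a configurable collision profile, sets movement velocity from direction and speed, and sanitizes the damage range.
; On hit, it sends a rounded random damage amount through an interface message, with its owner as dealer, then destroys itself.
; Tick prints the collision profile, with on-screen display controlled by a debug flag.
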(event `self.ReceiveBeginPlay`
  (`|ExecutionSequence`
    (:`then_0`
      (`PrimitiveComponent.SetCollisionProfileName` (`self.Box`) (`self.CollisionProfileName`) true))
    (:`then_1`
      (set `MovementComponent.Velocity` (* (`self.Direction`) (`self.MoveSpeed`)) (`self.ProjectileMovement`)))
    (:`then_2`
      (`self.FixDamageMinMax`))))

(event `self.ReceiveTick`
  (params (DeltaSeconds :type "Float (single-precision)"))
  (`KismetSystemLibrary.PrintString` (`KismetStringLibrary.Conv_NameToString` (`PrimitiveComponent.GetCollisionProfileName` (`self.Box`))) (`self.ShowDebug?`) false (struct :`G` 0.66 :`B` 1.0 :`A` 1.0) 0.0))

(event `self.Box.OnComponentHit`
  (params (HitComponent :type "PrimitiveComponent Object Reference") (OtherActor :type "Actor Object Reference") (OtherComp :type "PrimitiveComponent Object Reference") (NormalImpulse :type "Vector Structure") (Hit :type "HitResult Structure (by ref)"))
  (`self.On Hit` OtherActor))

(fn `FixDamageMinMax`
  (locals (NewMin :type "Float (double-precision)") (NewMax :type "Float (double-precision)"))
  (bind (_damageminmax_x _damageminmax_y) (`KismetMathLibrary.BreakVector2D` (`self.DamageMinMax`)))
  (bind _damageminmax_x_2 (`KismetMathLibrary.BreakVector2D` (`self.DamageMinMax`)))
  (bind (_damageminmax_x_3 _damageminmax_y_2) (`KismetMathLibrary.BreakVector2D` (`self.DamageMinMax`)))
  (`|ExecutionSequence`
    (:`then_0`
      (if (> _damageminmax_x_3 _damageminmax_y_2)
        (set `self.DamageMinMax` (`KismetMathLibrary.MakeVector2D` _damageminmax_y _damageminmax_y))))
    (:`then_1`
      (if (< _damageminmax_x_2 0.0)
        (set `self.DamageMinMax` (`KismetMathLibrary.MakeVector2D` 0.0 _damageminmax_y))))))

(fn `On Hit`
  (params (HitActor :type "Object Object Reference"))
  (returns (`HitSuccess?` :type Boolean))
  (bind (_damageminmax_x _damageminmax_y) (`KismetMathLibrary.BreakVector2D` (`self.DamageMinMax`)))
  (message `/Game/Dev_Content/Blueprints/Interfaces/BPI_Damageable.TakeDamage` HitActor (`KismetMathLibrary.Conv_IntToDouble` (`KismetMathLibrary.Round` (`KismetMathLibrary.RandomFloatInRange` _damageminmax_x _damageminmax_y))) (`self.GetOwner`))
  (`self.K2_DestroyActor`)
  (return (`KismetSystemLibrary.DoesImplementInterface` HitActor "/Game/Dev_Content/Blueprints/Interfaces/BPI_Damageable.BPI_Damageable_C")))

(fn `UserConstructionScript`)