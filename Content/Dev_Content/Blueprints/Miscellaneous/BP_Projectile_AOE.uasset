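; Projectile that deals direct damage on hit, then explodes for area-of-effect damage.
; On Hit sends randomized damage, hides the visuals, disables box collision and returns whether the target implements BPI_Damageable.
; After a configurable delay, a sphere overlap applies one shared random damage roll to every actor found, printing damageable names.
; It can draw a debug circle for the radius, then destroys itself shortly afterward.
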(event `TriggerExplosion_Event`
  (`KismetSystemLibrary.Delay` (`self.Delay`))
  (bind _outactors (`KismetSystemLibrary.SphereOverlapActors` (`self.K2_GetActorLocation`) (`self.Radius`) (`self.HittableObjects`)))
  (`self.ApplyAOEDamage` _outactors)
  (`self.Draw_AOE_Debug` (`self.ShowDebug?`))
  (`self.Event_DelayedDestroy` 0.1))

(event `Draw_AOE_Debug`
  (params (`Draw?` :type Boolean))
  (if `Draw?`
    (`KismetSystemLibrary.DrawDebugCircle` (`self.K2_GetActorLocation`) (`self.Radius`) 40 (struct :`R` 1.0 :`G` 0.501961 :`A` 1.0) 1.0 3.0 (1.0 0.0 0.0) (0.0 1.0 0.0))))

(event `Event_DelayedDestroy`
  (params (Duration :type "Float (single-precision)"))
  (`KismetSystemLibrary.Delay` Duration)
  (`self.K2_DestroyActor`))

(fn `ApplyAOEDamage`
  (params (Array :type "Array of Actor Object Reference"))
  (locals (Damage :type "Float (double-precision)"))
  (bind (_aoe_damageminmax_x _aoe_damageminmax_y) (`KismetMathLibrary.BreakVector2D` (`self.AOE_DamageMinMax`)))
  (set `local.Damage` (`KismetMathLibrary.RandomFloatInRange` _aoe_damageminmax_x _aoe_damageminmax_y))
  (for _array_element Array
    (message `/Game/Dev_Content/Blueprints/Interfaces/BPI_Damageable.TakeDamage` _array_element (`local.Damage`) (`self.GetOwner`))
    (if (`KismetSystemLibrary.DoesImplementInterface` _array_element "/Game/Dev_Content/Blueprints/Interfaces/BPI_Damageable.BPI_Damageable_C")
      (`KismetSystemLibrary.PrintString` (`KismetSystemLibrary.GetDisplayName` _array_element) true false (struct :`G` 0.66 :`B` 1.0 :`A` 1.0) 4.0))))

(fn `On Hit`
  (params (HitActor :type "Object Object Reference"))
  (returns (`HitSuccess?` :type Boolean))
  (bind (_damageminmax_x _damageminmax_y) (`KismetMathLibrary.BreakVector2D` (`self.DamageMinMax`)))
  (message `/Game/Dev_Content/Blueprints/Interfaces/BPI_Damageable.TakeDamage` HitActor (`KismetMathLibrary.Conv_IntToDouble` (`KismetMathLibrary.Round` (`KismetMathLibrary.RandomFloatInRange` _damageminmax_x _damageminmax_y))) (`self.GetOwner`))
  (`SceneComponent.SetVisibility` (`self.GFX Holder`) false true)
  (`self.TriggerExplosion_Event`)
  (`PrimitiveComponent.SetCollisionProfileName` (`self.Box`) "Nocollision" false)
  (return (`KismetSystemLibrary.DoesImplementInterface` HitActor "/Game/Dev_Content/Blueprints/Interfaces/BPI_Damageable.BPI_Damageable_C")))

(fn `UserConstructionScript`
  (`parent.UserConstructionScript`))