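; BP_FloatingText is an actor that shows a piece of floating text through its Widget and removes itself afterwards.
; On BeginPlay it passes its Text to the UI_FloatingText widget's ShowText and sets IsAnimated.
; While that flag is set, Tick polls the widget's IsDonePlaying and destroys the actor once it returns true.
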(event `self.ReceiveBeginPlay`
  (bind _asui_floating_text (cast `/Game/Dev_Content/Blueprints/UI/Misc/UI_FloatingText` (`WidgetComponent.GetWidget` (`self.Widget`))))
  (`/Game/Dev_Content/Blueprints/UI/Misc/UI_FloatingText.ShowText` _asui_floating_text (`self.Text`))
  (set `self.IsAnimated` true))

(event `self.ReceiveTick`
  (params (DeltaSeconds :type "Float (single-precision)"))
  (if (`self.IsAnimated`)
    (bind _asui_floating_text (cast `/Game/Dev_Content/Blueprints/UI/Misc/UI_FloatingText` (`WidgetComponent.GetWidget` (`self.Widget`))))
    (if (`/Game/Dev_Content/Blueprints/UI/Misc/UI_FloatingText.IsDonePlaying` _asui_floating_text)
      (`self.K2_DestroyActor`))))

(fn `UserConstructionScript`)