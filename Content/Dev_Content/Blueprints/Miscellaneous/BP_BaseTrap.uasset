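; BP_BaseTrap is a projectile-launched trap that stuns a status-effect-capable actor that overlaps it.
; It starts moving at an initial velocity, with its lifespan set in the construction script.
; A GroundCheck hit prints a debug message, disables GroundCheck collision and applies a configured collision profile to HitCheck.
; A HitCheck overlap with a BPI_StatusEffects actor adds a timed AC_Stun_SE, then destroys the trap.
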(event `self.ReceiveBeginPlay`
  (set `MovementComponent.Velocity` (`self.InitialVelocity`) (`self.ProjectileMovement`)))

(event `self.GroundCheck.OnComponentHit`
  (params (HitComponent :type "PrimitiveComponent Object Reference") (OtherActor :type "Actor Object Reference") (OtherComp :type "PrimitiveComponent Object Reference") (NormalImpulse :type "Vector Structure") (Hit :type "HitResult Structure (by ref)"))
  (`KismetSystemLibrary.PrintString` "Grounded")
  (`PrimitiveComponent.SetCollisionProfileName` (`self.HitCheck`) (`self.CollisionProfileName`) false)
  (`PrimitiveComponent.SetCollisionProfileName` (`self.GroundCheck`) "NoCollision" false))

(event `self.HitCheck.OnComponentBeginOverlap`
  (params (OverlappedComponent :type "PrimitiveComponent Object Reference") (OtherActor :type "Actor Object Reference") (OtherComp :type "PrimitiveComponent Object Reference") (OtherBodyIndex :type Integer) (bFromSweep :type Boolean) (SweepResult :type "HitResult Structure (by ref)"))
  (if (`KismetSystemLibrary.DoesImplementInterface` OtherActor "/Game/Dev_Content/Blueprints/Interfaces/BPI_StatusEffects.BPI_StatusEffects_C")
    (`|AddComponentByClass` OtherActor "/Game/Dev_Content/Blueprints/Components/StatusEffects/AC_Stun_SE.AC_Stun_SE_C" null 0.0 (`self.StunDuration`))
    (`self.K2_DestroyActor`)))

(fn `UserConstructionScript`
  (`self.SetLifeSpan` (`self.LifeSpan`)))