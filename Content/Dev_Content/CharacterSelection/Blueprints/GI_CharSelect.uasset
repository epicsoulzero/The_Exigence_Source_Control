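; GI_CharSelect is a game instance Blueprint that holds the player's character selection data.
; SaveCharacterData stores gender choice, mesh index, skin, top, pants and boots, plus anim classes for the game, clothing pieces and first-person arms.
; LoadCharacterData returns the same variables unchanged, including the first-person arms.
; The data lives only in instance variables, with no SaveGame or disk write.
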(event `/Game/Dev_Content/CharacterSelection/Blueprints/IF_CharSelect.SaveCharacterData`
  (params (MaleOrFemale :type Boolean) (SKMesh_Index :type Integer) (Skin :type "SkeletalMesh Object Reference") (CharTop :type "SkeletalMesh Object Reference") (CharPants :type "SkeletalMesh Object Reference") (CharBoots :type "SkeletalMesh Object Reference") (GameAnimClass :type "AnimInstance Class Reference") (TopAnimClass :type "AnimInstance Class Reference") (PantsAnimClass :type "AnimInstance Class Reference") (BootsAnimClass :type "AnimInstance Class Reference") (FPArms :type "SkeletalMesh Object Reference") (FPAnimCLass :type "AnimInstance Class Reference"))
  (set `self.MaleOrFemale` MaleOrFemale)
  (set `self.SkinIndex` SKMesh_Index)
  (set `self.Skin` Skin)
  (set `self.CharTop` CharTop)
  (set `self.CharPants` CharPants)
  (set `self.CharBoots` CharBoots)
  (set `self.GameAnimClass` GameAnimClass)
  (set `self.TopAnimClass` TopAnimClass)
  (set `self.PantsAnimClass` PantsAnimClass)
  (set `self.BootsAnimClass` BootsAnimClass)
  (set `self.FPArms` FPArms)
  (set `self.FPAnimClass` FPAnimCLass))

(fn `LoadCharacterData`
  (returns (MaleOrFemale :type Boolean) (SKMeshIndex :type Integer) (SKin :type "SkeletalMesh Object Reference") (CharTop :type "SkeletalMesh Object Reference") (CharPants :type "SkeletalMesh Object Reference") (CharBoots :type "SkeletalMesh Object Reference") (GameAnimClass :type "AnimInstance Class Reference") (TopAnimClass :type "AnimInstance Class Reference") (PantsAnimClass :type "AnimInstance Class Reference") (BootsAnimClass :type "AnimInstance Class Reference") (FPArms :type "SkeletalMesh Object Reference") (FPAnimClass :type "AnimInstance Class Reference"))
  (return (`self.MaleOrFemale`) (`self.SkinIndex`) (`self.Skin`) (`self.CharTop`) (`self.CharPants`) (`self.CharBoots`) (`self.GameAnimClass`) (`self.TopAnimClass`) (`self.PantsAnimClass`) (`self.BootsAnimClass`) (`self.FPArms`) (`self.FPAnimClass`)))