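; Character selection preview actor that creates the selection widget and lets the player pick gender, skin, tops, pants and boots.
; Cycle events swap meshes from male/female data arrays, with clothing following the body through master pose, and send choices to the Game Instance for saving.
; Timelines fade body dynamic materials, built at BeginPlay from data tables, through Opacity.
; Slider events drive rotation, camera height and face-socket-based zoom.
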(event `CycleTops`
  (params (Direction :type Integer))
  ;[1 1 1] Cycle through Tops so it matches character
  (`self.SetTopsMesh` Direction)
  (`self.UpdateCharacterData`))

(event `UpdateCharacterData`
  ;[1 1 1] Update Character Data/ Save what skeleton and Colors you pick to Game Instance to load on event begin play
  (`self.SetAndSaveCharacterData`))

(event `CyclePants`
  (params (Direction :type Integer))
  ;[1 1 1] Cycle through Pants so it matches character
  (`self.SetPantsMesh` Direction)
  (`self.UpdateCharacterData`))

(event `CycleBoots`
  (params (Direction :type Integer))
  ;[1 1 1] Cycle through Boots so it matches character
  (`self.SetBootsMesh` Direction)
  (`self.UpdateCharacterData`))

(event `CharacterFadeInTimer`
  ;[0.06007 0.1438 0.451 1 24] Non Replicated Events
  ;;[1 1 1] Set any material here for character so they fade in on timer
  (set `self.TimeLineNumber` 0)
  (`self.SetCharacter`)
  (`self.SetPantsMesh` 0)
  (`self.SetBootsMesh` 0)
  (`self.SetTopsMesh` 0))

(event `self.ReceiveTick`
  (params (DeltaSeconds :type "Float (single-precision)"))
  ;[0.06007 0.1438 0.451 1 24] Non Replicated Events
  ;;[1 1 1] Sliders
  (if (`self.FaceOrBody`) :!label _label
    (set `SpringArmComponent.SocketOffset` (`KismetMathLibrary.MakeVector` 0.0 0.0 (stale `Zoom` _returnvalue)) (`self.SpringArm`))))

(event `CameraHeight`
  (params (ZoomOffset :type "Float (double-precision)"))
  ;[0.06007 0.1438 0.451 1 24] Non Replicated Events
  ;;[1 1 1] Sliders
  (`self.CameraHeightSlider` ZoomOffset))

(event `Zoom`
  (params (Zoom :type "Float (double-precision)") (ZoomOffset :type "Float (double-precision)"))
  ;[0.06007 0.1438 0.451 1 24] Non Replicated Events
  ;;[1 1 1] Sliders
  (bind _returnvalue (`self.ZoomSlider` Zoom ZoomOffset))
  (goto _label))

(event `RotateCharacter`
  (params (Value :type "Float (double-precision)"))
  ;[0.06007 0.1438 0.451 1 24] Non Replicated Events
  ;;[1 1 1] Sliders
  (`self.CharacterRotationSlider` Value))

(event `self.ReceiveBeginPlay`
  (bind _returnvalue (`GameplayStatics.GetPlayerController` 0))
  (bind _returnvalue_2 (`GameplayStatics.GetPlayerController` 0))
  ;[1 1 1] Event Begin Play
  ;[1 1 1] Create and Fade in Character and selection widget
  (`|ExecutionSequence`
    (:`then_0`
      (`self.SetCharacterFade_MI`))
    (:`then_1`
      (`self.CharacterFadeInTimer`))
    (:`then_2`
      (`self.UpdateCharacterData`)
      ;;[1 1 1] Event for changing to idle or dance animations
      (`self.StartMenuAnims_ON_Off`)
      (`/Engine/EditorBlueprintResources/StandardMacros.IsValid` _returnvalue_2
        (:`Is Valid`
          (bind _returnvalue_3 (`|CreateWidget` "/Game/Dev_Content/CharacterSelection/Widgets/WB_CharSelect.WB_CharSelect_C" _returnvalue_2))
          (bind _output_get (set `self.CharSelect_WB` _returnvalue_3))
          (`UserWidget.PlayAnimation` _output_get (`/Game/Dev_Content/CharacterSelection/Widgets/WB_CharSelect.FadeIn` _output_get) 0.0 1 "Forward" 1.0 false)
          (set `self.BP_CharacterSelection` self)
          (`UserWidget.AddToViewport` _output_get 0)
          (set `PlayerController.bShowMouseCursor` true _returnvalue)
          (`WidgetBlueprintLibrary.SetInputMode_UIOnlyEx` _returnvalue (`self.CharSelect_WB`)))))))

(event `SelectGender`
  (params (IsMale :type Boolean))
  ;[1 1 1] Select Gender and set which is visible in selection screen
  (set `self.IsMale` IsMale)
  (`SceneComponent.SetVisibility` (`self.Female`) (not IsMale) false)
  (`SceneComponent.SetVisibility` (`self.FemaleTop`) (not IsMale) false)
  (`SceneComponent.SetVisibility` (`self.FemalePants`) (not IsMale) false)
  (`SceneComponent.SetVisibility` (`self.FemaleBoots`) (not IsMale) false)
  (`SceneComponent.SetVisibility` (`self.Male`) (`self.IsMale`) false)
  (`SceneComponent.SetVisibility` (`self.MaleTop`) (`self.IsMale`) false)
  (`SceneComponent.SetVisibility` (`self.MalePants`) (`self.IsMale`) false)
  (`SceneComponent.SetVisibility` (`self.MaleBoots`) (`self.IsMale`) false)
  (set `self.SkinIndex` (select `bool` (`self.IsMale`) :`false` (`.FemaleSkinIndex_36_55FA688A45EA8CE787C33C92DF2765B2` (break `/Game/Dev_Content/CharacterSelection/Structs_Tables/Female_Struct` (`self.FemaleDT`))) :`true` (`.MaleSkinIndex_40_57EFF1EC4CB641A5F07E2187AD17A23E` (break `/Game/Dev_Content/CharacterSelection/Structs_Tables/Male_Struct` (`self.MaleDT`)))))
  (set `self.TimeLineNumber` 1)
  (`self.SetCharacter`))

(event `CycleSkin`
  (params (Direction :type Integer))
  (bind (_femaleskin _femaletop _femalepants _femaleboots _femaleskinindex) (break `/Game/Dev_Content/CharacterSelection/Structs_Tables/Female_Struct` (`self.FemaleDT`)))
  (bind (_maleskin _maletop _malepants _maleboots _maleskinindex) (break `/Game/Dev_Content/CharacterSelection/Structs_Tables/Male_Struct` (`self.MaleDT`)))
  (bind _returnvalue (select `bool` (`self.IsMale`) :`false` _femaleskinindex :`true` _maleskinindex))
  (bind _returnvalue_2 (`KismetArrayLibrary.Array_Length` (select `bool` (`self.IsMale`) :`false` _femaleskin :`true` _maleskin)))
  (bind _returnvalue_3 (mod (+ _returnvalue Direction) _returnvalue_2))
  ;[1 1 1] Cycle Skin/Skeleton
  ;;[1 1 1] Cycle forward or backwards through characters
  (`|VariableSetRef` _returnvalue (select `bool` (< _returnvalue_3 0) :`false` _returnvalue_3 :`true` (- _returnvalue_2 1)))
  (set `self.SkinIndex` _returnvalue)
  (set `self.TimeLineNumber` 1)
  (`self.SetCharacter`))

(event `SetCharacter`
  (bind _skinindex (`self.SkinIndex`))
  (bind _skinindex_2 (`self.SkinIndex`))
  (bind _skinindex_3 (`self.SkinIndex`))
  (bind (_maleskin _maletop _malepants _maleboots _maleskinindex _maletopindex _malepantsindex _malebootsindex _malegameanimclass _maleidleanim _maledancinganim) (break `/Game/Dev_Content/CharacterSelection/Structs_Tables/Male_Struct` (`self.MaleDT`)))
  (bind (_femaleskin _femaletop _femalepants _femaleboots _femaleskinindex _femaletopindex _femalepantsindex _femalebootsindex _femalegameanimclass _femaleidleanim _femaledancinganim) (break `/Game/Dev_Content/CharacterSelection/Structs_Tables/Female_Struct` (`self.FemaleDT`)))
  ;[1 1 1] Set Character
  (if (`self.IsMale`)
    (for (_array_element _array_index) (`.MaleDMI_3_6BDE107A41AD1177F34748B105AD8663` (break `/Game/Dev_Content/CharacterSelection/Structs_Tables/MaleInstance` (`|GetArrayItem` (`self.MaleInstance`) _skinindex_3)))
      (`PrimitiveComponent.SetMaterial` (`self.Male`) _array_index _array_element))
    (else
      (for (_array_element_2 _array_index_2) (`.FemaleDMI_3_AD8B8A1644888AAE71A6549C946BC0C5` (break `/Game/Dev_Content/CharacterSelection/Structs_Tables/FemaleInstance` (`|GetArrayItem` (`self.FemaleInstance`) _skinindex_3)))
        (`PrimitiveComponent.SetMaterial` (`self.Female`) _array_index_2 _array_element_2))))
  (`SkinnedMeshComponent.SetSkinnedAssetAndUpdate` (select `bool` (`self.IsMale`) :`false` (`self.Female`) :`true` (`self.Male`)) (`|GetArrayItem` (select `bool` (`self.IsMale`) :`false` (`.FemaleSkin_23_1D6968DA4F9BAA54968B51A3E3764D93` (break `/Game/Dev_Content/CharacterSelection/Structs_Tables/Female_Struct` (`self.FemaleDT`))) :`true` (`.MaleSkin_36_8EF40B1D42A36D65283F538F254D2ED0` (break `/Game/Dev_Content/CharacterSelection/Structs_Tables/Male_Struct` (`self.MaleDT`)))) (`self.SkinIndex`)) true)
  (`self.UpdateCharacterData`)
  (if (`self.Anims_On_Off?`)
    (`SkeletalMeshComponent.SetAnimInstanceClass` (`self.Male`) (select `bool` (`self.IsMale`) :`false` (`|GetArrayItem` _femaledancinganim _skinindex_2) :`true` (`|GetArrayItem` _maledancinganim _skinindex_2)))
    (`SkeletalMeshComponent.SetAnimInstanceClass` (`self.Female`) (select `bool` (`self.IsMale`) :`false` (`|GetArrayItem` _femaledancinganim _skinindex_2) :`true` (`|GetArrayItem` _maledancinganim _skinindex_2)))
    (else
      (`SkeletalMeshComponent.SetAnimInstanceClass` (`self.Male`) (select `bool` (`self.IsMale`) :`false` (`|GetArrayItem` _femaleidleanim _skinindex) :`true` (`|GetArrayItem` _maleidleanim _skinindex)))
      (`SkeletalMeshComponent.SetAnimInstanceClass` (`self.Female`) (select `bool` (`self.IsMale`) :`false` (`|GetArrayItem` _femaleidleanim _skinindex) :`true` (`|GetArrayItem` _maleidleanim _skinindex)))))
  (switch `int` (`self.TimeLineNumber`)
    (:`0`
      (bind (_direction _newtrack_1) (`Timeline|BeginPlay` :!via `PlayFromStart`)
        (:`Update`
          (for _array_element_3 (`MeshComponent.GetMaterials` (select `bool` (`self.IsMale`) :`false` (`self.Female`) :`true` (`self.Male`)))
            (bind _asmaterial_instance_dynamic (cast `MaterialInstanceDynamic` _array_element_3))
            (`MaterialInstanceDynamic.SetScalarParameterValue` _asmaterial_instance_dynamic "Opacity" _newtrack_1)))))
    (:`1`
      (bind (_direction_2 _newtrack_0) (`Timeline|SwitchCharacter` :!via `PlayFromStart`)
        (:`Update`
          (for _array_element_4 (`MeshComponent.GetMaterials` (select `bool` (`self.IsMale`) :`false` (`self.Female`) :`true` (`self.Male`)))
            (bind _asmaterial_instance_dynamic_2 (cast `MaterialInstanceDynamic` _array_element_4))
            (`MaterialInstanceDynamic.SetScalarParameterValue` _asmaterial_instance_dynamic_2 "Opacity" _newtrack_0)))))))

(event `FadeItem`
  (params (Target :type "MaterialInstanceDynamic Object Reference"))
  (bind (_direction _newtrack_0) (`Timeline|Timeline_0` :!via `PlayFromStart`)
    (:`Update`
      (`/Engine/EditorBlueprintResources/StandardMacros.IsValid` Target
        (:`Is Valid`
          (`MaterialInstanceDynamic.SetScalarParameterValue` Target "Opacity" _newtrack_0))))))

(fn `CameraHeightSlider`
  (params (Value :type "Float (double-precision)"))
  (if (not (`self.FaceOrBody`))
    (set `SpringArmComponent.SocketOffset` (`KismetMathLibrary.MakeVector` 0.0 0.0 (`KismetMathLibrary.MapRangeClamped` Value 0.0 1.0 -94.0 50.0)) (`self.SpringArm`))))

(fn `CharacterRotationSlider`
  (params (Value :type "Float (double-precision)"))
  (`SceneComponent.K2_SetWorldRotation` (`self.Male`) (`KismetMathLibrary.MakeRotator` 0.0 0.0 (`KismetMathLibrary.MapRangeClamped` Value 0.0 1.0 0.0 360.0)) false false)
  (`SceneComponent.K2_SetWorldRotation` (`self.Female`) (`KismetMathLibrary.MakeRotator` 0.0 0.0 (`KismetMathLibrary.MapRangeClamped` Value 0.0 1.0 0.0 360.0)) false false))

(fn `SetAndSaveCharacterData`
  (bind (_femaleskin _femaletop _femalepants _femaleboots _femaleskinindex _femaletopindex _femalepantsindex _femalebootsindex _femalegameanimclass _femaleidleanim _femaledancinganim _femaletopanim _femalepantsanim _femalebootsanim _femalefparms _femalefpanimclass) (break `/Game/Dev_Content/CharacterSelection/Structs_Tables/Female_Struct` (`self.FemaleDT`)))
  (bind (_maleskin _maletop _malepants _maleboots _maleskinindex _maletopindex _malepantsindex _malebootsindex _malegameanimclass _maleidleanim _maledancinganim _maletopanim _malepantsanim _malebootsanim _malefparms _malefpanimclass) (break `/Game/Dev_Content/CharacterSelection/Structs_Tables/Male_Struct` (`self.MaleDT`)))
  (message `/Game/Dev_Content/CharacterSelection/Blueprints/IF_CharSelect.SaveCharacterData` (`GameplayStatics.GetGameInstance`) (`self.IsMale`) (select `bool` (`self.IsMale`) :`false` _maleskinindex :`true` _femaleskinindex) (select `bool` (`self.IsMale`) :`false` (`|GetArrayItem` _femaleskin _femaleskinindex) :`true` (`|GetArrayItem` _maleskin _maleskinindex)) (select `bool` (`self.IsMale`) :`false` (`|GetArrayItem` _femaletop _femaleskinindex) :`true` (`|GetArrayItem` _maletop _maleskinindex)) (select `bool` (`self.IsMale`) :`false` (`|GetArrayItem` _femalepants _femaleskinindex) :`true` (`|GetArrayItem` _malepants _maleskinindex)) (select `bool` (`self.IsMale`) :`false` (`|GetArrayItem` _femaleboots _femaleskinindex) :`true` (`|GetArrayItem` _maleboots _maleskinindex)) (select `bool` (`self.IsMale`) :`false` (`|GetArrayItem` _femalegameanimclass _femaleskinindex) :`true` (`|GetArrayItem` _malegameanimclass _maleskinindex)) (select `bool` (`self.IsMale`) :`false` (`|GetArrayItem` _femaletopanim _femaletopindex)) (select `bool` (`self.IsMale`) :`false` (`|GetArrayItem` _femalepantsanim _femalepantsindex) :`true` (`|GetArrayItem` _malepantsanim _malepantsindex)) (select `bool` (`self.IsMale`) :`false` (`|GetArrayItem` _femalebootsanim _femalebootsindex) :`true` (`|GetArrayItem` _malebootsanim _malebootsindex)) (select `bool` (`self.IsMale`) :`false` (`|GetArrayItem` _femalefparms _femaleskinindex) :`true` (`|GetArrayItem` _malefparms _maleskinindex)) (select `bool` (`self.IsMale`) :`false` (`|GetArrayItem` _femalefpanimclass _femaleskinindex) :`true` (`|GetArrayItem` _malefpanimclass _maleskinindex))))

(fn `SetBootsMesh`
  (params (Direction :type Integer))
  (bind _ismale (`self.IsMale`))
  (bind (_femaleskin _femaletop _femalepants _femaleboots _femaleskinindex _femaletopindex _femalepantsindex _femalebootsindex) (break `/Game/Dev_Content/CharacterSelection/Structs_Tables/Female_Struct` (`self.FemaleDT`)))
  (bind (_maleskin _maletop _malepants _maleboots _maleskinindex _maletopindex _malepantsindex _malebootsindex) (break `/Game/Dev_Content/CharacterSelection/Structs_Tables/Male_Struct` (`self.MaleDT`)))
  (bind _returnvalue (select `bool` (`self.IsMale`) :`false` _femaleboots :`true` _maleboots))
  (bind _returnvalue_2 (select `bool` (`self.IsMale`) :`false` _femalebootsindex :`true` _malebootsindex))
  (bind _returnvalue_3 (`KismetArrayLibrary.Array_Length` _returnvalue))
  (bind _returnvalue_4 (mod (+ _returnvalue_2 Direction) _returnvalue_3))
  (`|VariableSetRef` _returnvalue_2 (select `bool` (< _returnvalue_4 0) :`false` _returnvalue_4 :`true` (- _returnvalue_3 1)))
  (`SceneComponent.SetVisibility` (`self.MaleBoots`) _ismale false)
  (`SceneComponent.SetVisibility` (`self.FemaleBoots`) (not _ismale) false)
  (`SkinnedMeshComponent.SetSkinnedAssetAndUpdate` (select `bool` (`self.IsMale`) :`false` (`self.FemaleBoots`) :`true` (`self.MaleBoots`)) (`|GetArrayItem` _returnvalue _returnvalue_2) true))

(fn `SetCharacterFade_MI`
  (locals (DMI :type "Array of MaterialInstanceDynamic Object Reference") (PantsDMI :type "Array of MaterialInstanceDynamic Object Reference"))
  ;[1 1 1] Order of character has to be same as skin array  (Count starts from 1st male to last male then 1st female to last female)--(set only 1st material if you only have one mat on character and leave the rest to blank/select asset no need to disconnect as an isvalid node checks so it ok to leave blank)
  (`|ExecutionSequence`
    (:`then_0`
      (bind _outrownames (`DataTableFunctionLibrary.GetDataTableRowNames` "/Game/Dev_Content/CharacterSelection/Structs_Tables/MaleMaterials_DT.MaleMaterials_DT"))
      (for _array_element _outrownames
        (bind _returnvalue (`|GetDataTableRow` "/Game/Dev_Content/CharacterSelection/Structs_Tables/MaleMaterials_DT.MaleMaterials_DT" _array_element)
          (:`then`
            (bind _returnvalue_2 (`KismetArrayLibrary.Array_AddUnique` (`self.MaleMaterials`) _returnvalue))
            (for _array_element_2 (`.MaleMaterialInstance_3_B0BB575E4088959A8616C69C10B60CEC` (break `/Game/Dev_Content/CharacterSelection/Structs_Tables/MaleMaterialStruct` _returnvalue))
              (bind _returnvalue_3 (`KismetMaterialLibrary.CreateDynamicMaterialInstance` _array_element_2))
              (`KismetArrayLibrary.Array_AddUnique` (`local.DMI`) _returnvalue_3))
            (`KismetArrayLibrary.Array_Set` (`self.MaleInstance`) _returnvalue_2 (make `/Game/Dev_Content/CharacterSelection/Structs_Tables/MaleInstance` (`local.DMI`)) true)
            (`KismetArrayLibrary.Array_Clear` (`local.DMI`))))))
    (:`then_1`
      (bind _outrownames_2 (`DataTableFunctionLibrary.GetDataTableRowNames` "/Game/Dev_Content/CharacterSelection/Structs_Tables/FemaleMaterials_DT.FemaleMaterials_DT"))
      (for _array_element_3 _outrownames_2
        (bind _returnvalue_4 (`|GetDataTableRow` "/Game/Dev_Content/CharacterSelection/Structs_Tables/FemaleMaterials_DT.FemaleMaterials_DT" _array_element_3)
          (:`then`
            (bind _returnvalue_5 (`KismetArrayLibrary.Array_AddUnique` (`self.FemaleMaterials`) _returnvalue_4))
            (for _array_element_4 (`.FemaleMaterialInstance_3_F8885CB3490620D3B0C3959FFDDF42FE` (break `/Game/Dev_Content/CharacterSelection/Structs_Tables/FemaleMaterialStruct` _returnvalue_4))
              (bind _returnvalue_6 (`KismetMaterialLibrary.CreateDynamicMaterialInstance` _array_element_4))
              (`KismetArrayLibrary.Array_AddUnique` (`local.DMI`) _returnvalue_6))
            (`KismetArrayLibrary.Array_Set` (`self.FemaleInstance`) _returnvalue_5 (make `/Game/Dev_Content/CharacterSelection/Structs_Tables/FemaleInstance` (`local.DMI`)) true)
            (`KismetArrayLibrary.Array_Clear` (`local.DMI`))))))))

(fn `SetPantsMesh`
  (params (Direction :type Integer))
  (bind _ismale (`self.IsMale`))
  (bind (_femaleskin _femaletop _femalepants _femaleboots _femaleskinindex _femaletopindex _femalepantsindex) (break `/Game/Dev_Content/CharacterSelection/Structs_Tables/Female_Struct` (`self.FemaleDT`)))
  (bind (_maleskin _maletop _malepants _maleboots _maleskinindex _maletopindex _malepantsindex) (break `/Game/Dev_Content/CharacterSelection/Structs_Tables/Male_Struct` (`self.MaleDT`)))
  (bind _returnvalue (select `bool` (`self.IsMale`) :`false` _femalepantsindex :`true` _malepantsindex))
  (bind _returnvalue_2 (select `bool` (`self.IsMale`) :`false` _femalepants :`true` _malepants))
  (bind _returnvalue_3 (`KismetArrayLibrary.Array_Length` _returnvalue_2))
  (bind _returnvalue_4 (mod (+ _returnvalue Direction) _returnvalue_3))
  (`|VariableSetRef` _returnvalue (select `bool` (< _returnvalue_4 0) :`false` _returnvalue_4 :`true` (- _returnvalue_3 1)))
  (`SceneComponent.SetVisibility` (`self.MalePants`) _ismale false)
  (`SceneComponent.SetVisibility` (`self.FemalePants`) (not _ismale) false)
  (`SkinnedMeshComponent.SetSkinnedAssetAndUpdate` (select `bool` (`self.IsMale`) :`false` (`self.FemalePants`) :`true` (`self.MalePants`)) (`|GetArrayItem` _returnvalue_2 _returnvalue) true))

(fn `SetTopsMesh`
  (params (Direction :type Integer))
  (bind _ismale (`self.IsMale`))
  (bind (_femaleskin _femaletop _femalepants _femaleboots _femaleskinindex _femaletopindex) (break `/Game/Dev_Content/CharacterSelection/Structs_Tables/Female_Struct` (`self.FemaleDT`)))
  (bind (_maleskin _maletop _malepants _maleboots _maleskinindex _maletopindex) (break `/Game/Dev_Content/CharacterSelection/Structs_Tables/Male_Struct` (`self.MaleDT`)))
  (bind _returnvalue (select `bool` (`self.IsMale`) :`false` _femaletop :`true` _maletop))
  (bind _returnvalue_2 (select `bool` (`self.IsMale`) :`false` _femaletopindex :`true` _maletopindex))
  (bind _returnvalue_3 (`KismetArrayLibrary.Array_Length` _returnvalue))
  (bind _returnvalue_4 (mod (+ _returnvalue_2 Direction) _returnvalue_3))
  (`|VariableSetRef` _returnvalue_2 (select `bool` (< _returnvalue_4 0) :`false` _returnvalue_4 :`true` (- _returnvalue_3 1)))
  (`SceneComponent.SetVisibility` (`self.MaleTop`) _ismale false)
  (`SceneComponent.SetVisibility` (`self.FemaleTop`) (not _ismale) false)
  (`SkinnedMeshComponent.SetSkinnedAssetAndUpdate` (select `bool` (`self.IsMale`) :`false` (`self.FemaleTop`) :`true` (`self.MaleTop`)) (`|GetArrayItem` _returnvalue _returnvalue_2) true))

(fn `StartMenuAnims_ON_Off`
  (bind (_femaleskin _femaletop _femalepants _femaleboots _femaleskinindex _femaletopindex _femalepantsindex _femalebootsindex _femalegameanimclass _femaleidleanim _femaledancinganim) (break `/Game/Dev_Content/CharacterSelection/Structs_Tables/Female_Struct` (`self.FemaleDT`)))
  (bind (_maleskin _maletop _malepants _maleboots _maleskinindex _maletopindex _malepantsindex _malebootsindex _malegameanimclass _maleidleanim _maledancinganim) (break `/Game/Dev_Content/CharacterSelection/Structs_Tables/Male_Struct` (`self.MaleDT`)))
  ;[1 1 1] Sets what anim Class male and female have for Idle and Dance Animations
  (if (`self.Anims_On_Off?`)
    (`SkeletalMeshComponent.SetAnimInstanceClass` (`self.Male`) (select `bool` (`self.IsMale`) :`false` (`|GetArrayItem` _femaledancinganim _femaleskinindex) :`true` (`|GetArrayItem` _maledancinganim _maleskinindex)))
    (`SkeletalMeshComponent.SetAnimInstanceClass` (`self.Female`) (select `bool` (`self.IsMale`) :`false` (`|GetArrayItem` _femaledancinganim _femaleskinindex) :`true` (`|GetArrayItem` _maledancinganim _maleskinindex)))
    (else
      (`SkeletalMeshComponent.SetAnimInstanceClass` (`self.Male`) (select `bool` (`self.IsMale`) :`false` (`|GetArrayItem` _femaleidleanim _femaleskinindex) :`true` (`|GetArrayItem` _maleidleanim _maleskinindex)))
      (`SkeletalMeshComponent.SetAnimInstanceClass` (`self.Female`) (select `bool` (`self.IsMale`) :`false` (`|GetArrayItem` _femaleidleanim _femaleskinindex) :`true` (`|GetArrayItem` _maleidleanim _maleskinindex))))))

(fn `UserConstructionScript`
  (`SkinnedMeshComponent.SetLeaderPoseComponent` (`self.MaleTop`) (`self.Male`) false)
  (`SkinnedMeshComponent.SetLeaderPoseComponent` (`self.MalePants`) (`self.Male`) false)
  (`SkinnedMeshComponent.SetLeaderPoseComponent` (`self.MaleBoots`) (`self.Male`) false)
  (`SkinnedMeshComponent.SetLeaderPoseComponent` (`self.FemalePants`) (`self.Female`) false)
  (`SkinnedMeshComponent.SetLeaderPoseComponent` (`self.FemaleTop`) (`self.Female`) false)
  (`SkinnedMeshComponent.SetLeaderPoseComponent` (`self.FemaleBoots`) (`self.Female`) false))

(fn `ZoomSlider`
  (params (ValueZoom :type "Float (double-precision)") (ValueZoomOffset :type "Float (double-precision)"))
  (returns (ReturnValue :type "Float (double-precision)"))
  (set `SpringArmComponent.TargetArmLength` (`KismetMathLibrary.MapRangeClamped` ValueZoom 0.0 1.0 300.0 (`self.ZoomDistance`)) (`self.SpringArm`))
  (return (`KismetMathLibrary.MapRangeClamped` ValueZoomOffset 0.0 1.0 0.0 (- (.z (.location (`SceneComponent.GetSocketTransform` (select `bool` (`self.IsMale`) :`false` (`self.Male`) :`true` (`self.Female`)) "FaceSocket" "RTS_Component"))) 100.0))))