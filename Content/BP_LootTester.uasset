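; BP_LootTester is a test actor that spawns a batch of BP_Loot every three seconds on a ring around itself.
; Spawn points take a random direction scaled by HorizontalOffset and raised by VerticalOffset.
; With UseNoClipCheck on, WorldStatic sphere traces re-roll points that hit existing loot, up to an iteration cap.
; Tick draws the ring as a debug circle.
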(event `self.ReceiveBeginPlay`
  (`KismetSystemLibrary.RetriggerableDelay` 3.0 :!label _label)
  (`self.Event_SpawnLoot`)
  (goto _label))

(event `Event_SpawnLoot`
  (for _ (range 1 (+ (`self.LootCount`) 1))
    (`|SpawnActorFromClass` "/Game/BP_Loot.BP_Loot_C" (`KismetMathLibrary.MakeTransform` (select `bool` (`self.UseNoClipCheck?`) :`false` (`self.GetRandomSpawnPoint`) :`true` (`self.GetNoClipSpawnPoints` 50.0 50))) "AlwaysSpawn" "OverrideRootScale" null null)))

(event `self.ReceiveTick`
  (params (DeltaSeconds :type "Float (single-precision)"))
  (`self.Event_DrawDebug`))

(event `Event_DrawDebug`
  (`|ExecutionSequence`
    (:`then_0`
      (`KismetSystemLibrary.DrawDebugCircle` (`self.K2_GetActorLocation`) (`self.HorizontalOffset`) 30 (struct :`G` 1.0 :`B` 1.0 :`A` 1.0) 0.0 2.0 (1.0 0.0 0.0) (0.0 1.0 0.0) true))))

(fn `GetNoClipSpawnPoints`
  (params (CheckRadius :type "Float (double-precision)") (MaxIteration :type Integer :default 1))
  (returns (Out :type "Vector Structure"))
  (locals (PointToCheck :type "Vector Structure" :default (0.0 0.0 0.0)))
  (for _ (range 1 (+ MaxIteration 1))
    (bind _output_get (set `local.PointToCheck` (`self.GetRandomSpawnPoint`)))
    (bind (_outhit _returnvalue) (`KismetSystemLibrary.SphereTraceSingleForObjects` _output_get (* _output_get -1000.0) (`local.CheckRadius`) (`|MakeArray` "ObjectTypeQuery1" :!type "EObjectTypeQuery Enum")))
    (if _returnvalue
      (if (not (== (`GameplayStatics.GetObjectClass` (`.HitActor` (`GameplayStatics.BreakHitResult` _outhit))) "/Game/BP_Loot.BP_Loot_C"))
        (break))
      (else
        (break))))
  (return (`local.PointToCheck`)))

(fn `GetRandomSpawnPoint`
  (returns (Out :type "Vector Structure"))
  (bind (_returnvalue_x _returnvalue_y) (`KismetMathLibrary.BreakVector` (`KismetMathLibrary.RandomUnitVector`)))
  (return (+ (`self.K2_GetActorLocation`) (* (`KismetMathLibrary.Normal` (`KismetMathLibrary.MakeVector` _returnvalue_x _returnvalue_y)) (`self.HorizontalOffset`)) (`KismetMathLibrary.MakeVector` 0.0 0.0 (`self.VerticalOffset`)))))

(fn `UserConstructionScript`)